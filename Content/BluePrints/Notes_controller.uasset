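; Rhythm note controller that spawns Main_Nodes actors on cues from a test-music timeline.
; Tick plays the timeline, whose four directional fall events all pick random start and end points on the Z=0 plane within ±ScrL.
; Each spawned node receives both points and a velocity that covers the route in DelayTime.
; The cue direction is currently ignored, and the TempDir direction branches are unconnected.
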(event Custom|falling%20with%20pos%20set
  ;[1 1 1] spawn node
  (bind (_metatransform _speed) (CallFunction|Fuc#fallFrom# (stale EventTick _start_pos) (stale EventTick _end_pos) (Variables|Default|Getdelay_time)))
  (bind _returnvalue (Game|SpawnActorfromClass "/Game/BluePrints/Main_Nodes.Main_Nodes_C" _metatransform "AlwaysSpawn" 0 0))
  (Variables|/Game/BluePrints/Main_Nodes.Main_Nodes_C|Setspeed_of_Node _returnvalue _speed)
  (Variables|/Game/BluePrints/Main_Nodes.Main_Nodes_C|SetStart%20Pos _returnvalue (stale EventTick _start_pos))
  (Variables|/Game/BluePrints/Main_Nodes.Main_Nodes_C|SetTarget%20Pos _returnvalue (stale EventTick _end_pos)))

(event EventBeginPlay)

(event Collision|EventActorBeginOverlap
  (params (OtherActor :type Actor%20Object%20Reference)))

(event EventTick
  (params (DeltaSeconds :type Float%20%28single-precision%29))
  ;[1 1 1] emit spawning signal
  (Timeline|Timeline_test01 Play
    (:testMusic0%20fall_from_up
      _)
    (:testMusic0%20fall_from_down
      _)
    (:testMusic0%20fall_from_right
      _)
    (:testMusic0%20fall_from_left
      _))
  (bind (_start_pos _end_pos) (CallFunction|Fuc#randomLinearRoute#))
  ;[1 1 1] spawn node
  (bind (_metatransform _speed) (CallFunction|Fuc#fallFrom# _start_pos _end_pos (Variables|Default|Getdelay_time)))
  (bind _returnvalue (Game|SpawnActorfromClass "/Game/BluePrints/Main_Nodes.Main_Nodes_C" _metatransform "AlwaysSpawn" 0 0))
  (Variables|/Game/BluePrints/Main_Nodes.Main_Nodes_C|Setspeed_of_Node _returnvalue _speed)
  (Variables|/Game/BluePrints/Main_Nodes.Main_Nodes_C|SetStart%20Pos _returnvalue _start_pos)
  (Variables|/Game/BluePrints/Main_Nodes.Main_Nodes_C|SetTarget%20Pos _returnvalue _end_pos))

(fn ConstructionScript)

(fn Fuc#fallFrom#
  (params (start%20pos :type Vector) (tarrget%20pos :type Vector) (delay%20time%20%28local%29 :type Float%20%28single-precision%29))
  (bind _output_get (LocalVariables|Setspawn%20SPD (/ (- tarrget%20pos start%20pos) delay%20time%20%28local%29)))
  (return (Math|Transform|MakeTransform start%20pos) _output_get))

(fn Fuc#randomLinearRoute#
  (return (Math|Vector|MakeVector (Math|Random|RandomFloatinRange (* (Variables|Default|GetScr_L) -1.0) (Variables|Default|GetScr_L)) (Math|Random|RandomFloatinRange (* (Variables|Default|GetScr_L) -1.0) (Variables|Default|GetScr_L)) 0.0) (Math|Vector|MakeVector (Math|Random|RandomFloatinRange (* (Variables|Default|GetScr_L) -1.0) (Variables|Default|GetScr_L)) (Math|Random|RandomFloatinRange (* (Variables|Default|GetScr_L) -1.0) (Variables|Default|GetScr_L)) 0.0)))