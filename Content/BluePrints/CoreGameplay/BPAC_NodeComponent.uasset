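; Actor component that moves its owning actor, apparently a note (per its error text), at a constant velocity and tracks its travel progress.
; Each Tick offsets the owner's location by SpeedOfNode scaled by delta time, without sweeping, and prints an error if the move fails.
; After a successful move, Progress becomes distance from StartPos over the StartPos-to-TargetPos distance, capped slightly past 1 to allow overshoot.
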(event EventBeginPlay)

(event EventTick
  (params (DeltaSeconds :type Float%20%28single-precision%29))
  (CallFunction|Func#move# DeltaSeconds))

(fn Func#updateProgress#
  (Variables|Default|SetProgress (Math|Float|Min(Float) (/ (Math|Vector|VectorLength (- (Transformation|GetActorLocation (Components|GetOwner)) (Variables|Default|GetStart%20Pos))) (Math|Vector|VectorLength (- (Variables|Default|GetTarget%20Pos) (Variables|Default|GetStart%20Pos)))) 1.1)))

(fn Func#move#
  (params (delta%20time :type Float%20%28single-precision%29))
  (bind _returnvalue (Transformation|SetActorLocation (Components|GetOwner) (+ (Transformation|GetActorLocation (Components|GetOwner)) (* (Variables|Default|GetSpeed%20of%20node) delta%20time)) false false))
  (if _returnvalue
    (CallFunction|Func#updateProgress#)
    (else
      (Development|PrintString "Note Movement Error"))))