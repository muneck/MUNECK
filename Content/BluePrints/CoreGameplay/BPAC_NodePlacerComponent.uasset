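; An actor component that places rhythm-game notes on keyed rails so they travel toward the rail end.
; It looks up the rail's start, end and note transform in the level variable component, converting both endpoints with VportScaled2map.
; Velocity is the start-to-end offset divided by delay time.
; It spawns the class mapped to the note type and attaches a BPAC_NodeComponent carrying start, target and speed.
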(event EventTick
  (params (DeltaSeconds :type Float%20%28single-precision%29)))

(fn Fuc#placeNoteonRoute#
  (params (Key%20of%20track :type Integer) (Node_Type :type E_NodeType%20Enum :default "NewEnumerator0") (delay%20time :type Float%20%28single-precision%29))
  (bind _spintransform (|CheckVaildandsavetolocalvariables Node_Type delay%20time Key%20of%20track))
  (bind (_metatransform _speed) (CallFunction|Fuc#fallFrom# (LocalVariables|GetNewNodeStartPos%28local%29) (LocalVariables|GetNewNodeTargetPos%28local%29) (LocalVariables|GetDelayTime%28local%29)))
  (LocalVariables|SetNewNodeSpeed%28local%29 _speed)
  ;[1 1 1] Spawn and init variables
  (bind _returnvalue (Game|SpawnActorfromClass (.Value (Utilities|Map|Find (Variables|Default|GetNodeTypeMap) (LocalVariables|GetNodeType%28local%29))) (Math|Transform|ComposeTransforms _spintransform _metatransform) "AlwaysSpawn" 0 0))
  (bind _returnvalue_2 (Game|AddComponentbyClass _returnvalue "/Game/BluePrints/CoreGameplay/BPAC_NodeComponent.BPAC_NodeComponent_C"))
  (Variables|/Game/BluePrints/CoreGameplay/BPAC_NodeComponent.BPAC_NodeComponent_C|SetStart%20Pos _returnvalue_2 (LocalVariables|GetNewNodeStartPos%28local%29))
  (Variables|/Game/BluePrints/CoreGameplay/BPAC_NodeComponent.BPAC_NodeComponent_C|SetSpeed%20of%20node _returnvalue_2 (LocalVariables|GetNewNodeSpeed%28local%29))
  (Variables|/Game/BluePrints/CoreGameplay/BPAC_NodeComponent.BPAC_NodeComponent_C|SetTarget%20Pos _returnvalue_2 (LocalVariables|GetNewNodeTargetPos%28local%29)))

(fn Fuc#fallFrom#
  (params (start%20pos :type Vector) (tarrget%20pos :type Vector) (delay%20time%20%28local%29 :type Float%20%28single-precision%29))
  (bind _output_get (LocalVariables|Setspawn%20SPD (/ (- tarrget%20pos start%20pos) delay%20time%20%28local%29)))
  (return (Math|Transform|MakeTransform start%20pos) _output_get))