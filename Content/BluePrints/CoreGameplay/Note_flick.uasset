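; Flick note actor, apparently for a rhythm game, that travels from a start position toward a target.
; Each Tick it moves without sweep by its speed vector scaled by delta time, printing an error if the move fails.
; After each successful move it updates Progress as distance from start over total start-to-target distance, capped slightly past the target.
; The Blueprint contains no input or hit-judgement logic.
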(event EventBeginPlay)

(event Collision|EventActorBeginOverlap
  (params (OtherActor :type Actor%20Object%20Reference)))

(event EventTick
  (params (DeltaSeconds :type Float%20%28single-precision%29))
  (bind _returnvalue (Transformation|SetActorLocation (+ (Transformation|GetActorLocation) (* (Variables|Default|GetSpeed%20of%20node) DeltaSeconds)) false false))
  (if _returnvalue
    (CallFunction|Func#updateProgress#)
    (else
      (Development|PrintString "Note Movement Error"))))

(fn ConstructionScript)

(fn Func#updateProgress#
  (Variables|Default|SetProgress (Math|Float|Min(Float) (/ (Math|Vector|VectorLength (- (Transformation|GetActorLocation) (Variables|Default|GetStart%20Pos))) (Math|Vector|VectorLength (- (Variables|Default|GetTarget%20Pos) (Variables|Default|GetStart%20Pos)))) 1.1)))