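; Rhythm-game note controller that loads a song's JSON chart and metadata, then times note spawns during play.
; On game start it sorts notes by appear time (StartTime minus DelayTime) and starts the clock at the earliest non-positive value.
; Once activated, Tick follows music time, or delta time while audio is inactive, starting music at zero and broadcasting notes within a 0.02 window.
; It follows BP_GameStateManager pause events and ends the game when music finishes.
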(event Custom|GameStart
  (bind _gi (CallFunction|GFuncGetGI))
  (bind _output_get (Variables|Default|SetGI _gi))
  (CallFunction|ParseChartMetadata (Utilities|String|Append (Variables|/Game/BluePrints/CoreGameplay/CoreGameplayGI.CoreGameplayGI_C|GetSongName _output_get) "/" (Variables|/Game/BluePrints/CoreGameplay/CoreGameplayGI.CoreGameplayGI_C|GetFileName _output_get)))
  (CallFunction|ParseSongMetadata (Variables|/Game/BluePrints/CoreGameplay/CoreGameplayGI.CoreGameplayGI_C|GetSongName _output_get)))

(event Custom|LifeEnds
  (params (Reset%20Game :type Boolean))
  (Actor|DestroyActor))

(event Custom|Resume
  (Variables|Status|SetGamePause false))

(event Custom|Pause
  (Variables|Status|SetGamePause true))

(event Custom|activate
  (Utilities|FlowControl|Gate true) ; enters at Open
)

(event Custom|ED_MusicEnd_Event_0
  (Variables|Status|SetHasMusicEnd true))

(event EventBeginPlay
  (bind _returnvalue (Actor|GetActorOfClass "/Game/BluePrints/CoreGameplay/BP_GameStateManager.BP_GameStateManager_C"))
  (bind _output_get (Variables|Default|SetGSM _returnvalue))
  (EventDispatchers|AssignEDGameStart _output_get (delegate Custom|GameStart))
  (EventDispatchers|BindEventtoEDNoteStartDropping _output_get (delegate Custom|activate))
  (EventDispatchers|AssignEDGamePause _output_get (delegate Custom|Pause))
  (EventDispatchers|AssignEDGameResume _output_get (delegate Custom|Resume))
  (EventDispatchers|AssignEDGameEnd _output_get (delegate Custom|LifeEnds))
  (bind _returnvalue_2 (Game|SpawnActorfromClass "/Game/BluePrints/CoreGameplay/Load_Music/BP_music_loader.BP_music_loader_C" (Math|Transform|MakeTransform "0, 0, 0") "AlwaysSpawn" 0 0))
  (bind _output_get_2 (Variables|Default|SetMusicLoaderRef _returnvalue_2))
  (EventDispatchers|AssignEDMusicEnd _output_get_2 (delegate Custom|ED_MusicEnd_Event_0)))

(event EventTick
  (params (DeltaSeconds :type Float%20%28single-precision%29))
  (Utilities|FlowControl|Gate true
    (:Exit
      (Utilities|MGetTickWorkingStatus
        (:Proceed%20Ticking
          ;[1 1 1] emit spawning signal
          (bind _returnvalue (CallFunction|TickandRefreshCurNote DeltaSeconds))
          ;[1 1 1] after tick updates, Start the music when offset is reached
          (if (>= (Variables|current|GetCurrentTick) 0.0)
            (if (Variables|Status|GetHasMusicStart)
              _
              (else
                (Default|GSMStartMusic (Variables|Default|GetGSM))
                (Variables|Status|SetHasMusicStart true))))
          (if _returnvalue
            (CallFunction|UnpackNote)
            (CallFunction|NotePlacementWrapper)))
        (:Music%20Ended
          ;[1 1 1] FIXME:both music and note end = end game
          (Default|GSMEndGame (Variables|Default|GetGSM) false))))))

(fn ConstructionScript)

(fn ParseChartMetadata
  (params (FileName :type String))
  (bind _ijsonobject (Class|IJsonBlueprintFunctionLibrary|LoadJsonStringfromFile (Utilities|String|Append (Class|KismetSystemLibrary|GetProjectContentDirectory) "Charts/" FileName)))
  (Variables|Data|SetChartObject _ijsonobject)
  (bind _outnumber (Class|IJsonObject|TryGetNumberField (Variables|Data|GetChartObject) "NoteNum"))
  (Variables|Data|SetNoteNum (Math|Float|Truncate _outnumber))
  (bind _ascore_gameplay_gi (Utilities|Casting|CastToCoreGameplayGI (Game|GetGameInstance)))
  (Variables|/Game/BluePrints/CoreGameplay/CoreGameplayGI.CoreGameplayGI_C|SetNoteNum _ascore_gameplay_gi (Variables|Data|GetNoteNum))
  (bind _outarray (Class|IJsonObject|TryGetJsonObjectArrayField (Variables|Data|GetChartObject) "NoteList"))
  (bind _output_get (Variables|Data|SetNoteList _outarray))
  (bind _sortednotelist (CallFunction|SortNoteList _output_get))
  (for _array_element _sortednotelist
    (bind _outnumber_2 (Class|IJsonObject|TryGetNumberField _array_element "StartTime"))
    (bind _outnumber_3 (Class|IJsonObject|TryGetNumberField _array_element "DelayTime"))
    (Variables|current|SetCurrentTick (Math|Float|Min(Float) (- _outnumber_2 _outnumber_3) (Variables|current|GetCurrentTick))))
  (for _array_element_2 (Variables|Data|GetNoteList)
    (bind _outnumber_4 (Class|IJsonObject|TryGetNumberField _array_element_2 "StartTime"))
    (bind _outnumber_5 (Class|IJsonObject|TryGetNumberField _array_element_2 "DelayTime"))
    (Utilities|Array|Add (Variables|Data|GetStartTimeList) (- _outnumber_4 _outnumber_5)))
  (Variables|Status|SetFinishedInit true))

(fn SortNoteList
  (params (NoteList :type Array%20of%20I%20Json%20Object%20Object%20References))
  (bind _returnvalue (Utilities|Array|Length NoteList))
  (bind _returnvalue_2 (- _returnvalue 2))
  (for _index (range 0 _returnvalue_2)
    (for _index_2 (range 0 (- _returnvalue_2 _index))
      (bind _appeartime (CallFunction|GetAppearTime (Utilities|Array|Get(acopy) NoteList _index_2)))
      (bind _appeartime_2 (CallFunction|GetAppearTime (Utilities|Array|Get(acopy) NoteList (+ _index_2 1))))
      (if (> _appeartime _appeartime_2)
        (Utilities|Array|Swap NoteList _index_2 (+ _index_2 1)))))
  (return NoteList))

(fn GetAppearTime
  (params (NoteObject :type I%20Json%20Object%20Object%20Reference))
  (bind _outnumber (Class|IJsonObject|TryGetNumberField NoteObject "StartTime"))
  (bind _outnumber_2 (Class|IJsonObject|TryGetNumberField NoteObject "DelayTime"))
  (return (- _outnumber _outnumber_2)))

(fn NotePlacementWrapper
  (Default|CallEDPlaceNode (Utilities|MMakeNodeInfo))
  (bind _output_get (Variables|Current|SetCurrentIndex (+ (Variables|Current|GetCurrentIndex) 1)))
  (Variables|Status|SetHasOverflowed (>= _output_get (Variables|Data|GetNoteNum))))

(fn TickandRefreshCurNote
  (params (DeltaSecs :type Float%20%28single-precision%29))
  (Utilities|MUpdateCurrentTick DeltaSecs)
  (return (< (Math|Float|Absolute(Float) (- (Variables|current|GetCurrentTick) (Utilities|Array|Get(acopy) (Variables|Data|GetStartTimeList) (Variables|Current|GetCurrentIndex)))) 0.02)))

(fn UnpackNote
  (bind _output_get (Variables|current|SetCurrentNote (Utilities|Array|Get(acopy) (Variables|Data|GetNoteList) (Variables|Current|GetCurrentIndex))))
  (bind _outstring (Class|IJsonObject|TryGetStringField _output_get "Type"))
  (Variables|Current|SetCurrentType _outstring)
  (bind _outnumber (Class|IJsonObject|TryGetNumberField (Variables|current|GetCurrentNote) "Rail"))
  (Variables|Current|SetCurrentRail (Math|Float|Truncate _outnumber))
  (bind _outnumber_2 (Class|IJsonObject|TryGetNumberField (Variables|current|GetCurrentNote) "Length"))
  (Variables|Current|SetCurrentLength _outnumber_2)
  (bind _outnumber_3 (Class|IJsonObject|TryGetNumberField (Variables|current|GetCurrentNote) "DelayTime"))
  (Variables|Current|SetCurrentDelayTime _outnumber_3)
  (bind _outnumber_4 (Class|IJsonObject|TryGetNumberField (Variables|current|GetCurrentNote) "StartTime"))
  (Variables|Current|SetCurrentStartTime _outnumber_4)
  (switch string ""
    (:flick
      (Utilities|Array|Add (Variables|/Game/BluePrints/CoreGameplay/CoreGameplayGI.CoreGameplayGI_C|GetNoteList (Variables|Default|GetGI)) (Utilities|Struct|MakeS_NoteInfo "NewEnumerator0" (Variables|Current|GetCurrentRail) (Variables|Current|GetCurrentLength) (Variables|Current|GetCurrentStartTime) (Variables|Current|GetCurrentDelayTime))))
    (:hold
      (Utilities|Array|Add (Variables|/Game/BluePrints/CoreGameplay/CoreGameplayGI.CoreGameplayGI_C|GetNoteList (Variables|Default|GetGI)) (Utilities|Struct|MakeS_NoteInfo "NewEnumerator1" (Variables|Current|GetCurrentRail) (Variables|Current|GetCurrentLength) (Variables|Current|GetCurrentStartTime) (Variables|Current|GetCurrentDelayTime))))
    (:avoid
      (Utilities|Array|Add (Variables|/Game/BluePrints/CoreGameplay/CoreGameplayGI.CoreGameplayGI_C|GetNoteList (Variables|Default|GetGI)) (Utilities|Struct|MakeS_NoteInfo "NewEnumerator2" (Variables|Current|GetCurrentRail) (Variables|Current|GetCurrentLength) (Variables|Current|GetCurrentStartTime) (Variables|Current|GetCurrentDelayTime))))))

(fn ParseSongMetadata
  (params (SongName :type String))
  (bind _output_get (Variables|Data|SetSongPath (Utilities|String|Append (Class|KismetSystemLibrary|GetProjectContentDirectory) "Charts/" SongName "/")))
  (bind _ijsonobject (Class|IJsonBlueprintFunctionLibrary|LoadJsonStringfromFile (Utilities|String|Append _output_get "meta.json")))
  (bind _output_get_2 (Variables|Data|SetSongObject _ijsonobject))
  (bind _outstring (Class|IJsonObject|TryGetStringField _output_get_2 "Name"))
  (bind _outstring_2 (Class|IJsonObject|TryGetStringField (Variables|Data|GetSongObject) "MusicFile"))
  (bind _outstring_3 (Class|IJsonObject|TryGetStringField (Variables|Data|GetSongObject) "IllustrationFile"))
  (bind _outstring_4 (Class|IJsonObject|TryGetStringField (Variables|Data|GetSongObject) "Artist"))
  (bind _outstring_5 (Class|IJsonObject|TryGetStringField (Variables|Data|GetSongObject) "Illustrator"))
  (bind _outnumber (Class|IJsonObject|TryGetNumberField (Variables|Data|GetSongObject) "ChartOffset"))
  (Variables|SongData|SetSongInfo (Utilities|Struct|MakeS_SongInfo _outstring _outstring_2 _outstring_3 _outstring_4 _outstring_5 _outnumber))
  (bind _outarray (Class|IJsonObject|TryGetJsonObjectArrayField (Variables|Data|GetSongObject) "Difficulties"))
  (bind _output_get_3 (Variables|SongData|SetDifficultyJsonList _outarray))
  (for _array_element _output_get_3
    (bind _outstring_6 (Class|IJsonObject|TryGetStringField _array_element "DifficultyName"))
    (bind _outnumber_2 (Class|IJsonObject|TryGetNumberField _array_element "Difficulty"))
    (bind _outstring_7 (Class|IJsonObject|TryGetStringField _array_element "ChartFileName"))
    (bind _outstring_8 (Class|IJsonObject|TryGetStringField _array_element "ChartDesigner"))
    (Utilities|Array|Add (Variables|SongData|GetDifficultyList) (Utilities|Struct|MakeS_SongDifficultyInfo _outstring_6 (Math|Float|Truncate _outnumber_2) _outstring_7 _outstring_8)))
  (Variables|/Game/BluePrints/CoreGameplay/CoreGameplayGI.CoreGameplayGI_C|SetSongInfo (Variables|Default|GetGI) (Variables|SongData|GetSongInfo))
  (Variables|/Game/BluePrints/CoreGameplay/CoreGameplayGI.CoreGameplayGI_C|SetSongDifficultyLIst (Variables|Default|GetGI) (Variables|SongData|GetDifficultyList)))