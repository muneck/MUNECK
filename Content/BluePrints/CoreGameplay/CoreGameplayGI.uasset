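; Game instance for a rhythm game that holds the selected song, its metadata and the score and combo state.
; On Init it sets a hardcoded song and chart file, then reads that song's meta.json from the Charts content folder.
; Parsing fills the song info struct and appends each difficulty to a list, then removes the list's first element.
; ResetScore zeroes score, combo and max combo.
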(event EventInit
  (Variables|inGame|Datas|SetSongName "StillAlive")
  (Variables|inGame|Datas|SetFileName "chart5.json")
  (CallFunction|ParseSongMetadata))

(fn ResetScore
  (Variables|inGame|GlobalVariables|SetScore 0.0)
  (Variables|inGame|GlobalVariables|SetCombo 0)
  (Variables|inGame|GlobalVariables|SetMaxCombo 0))

(fn ParseSongMetadata
  (bind _ijsonobject (Class|IJsonBlueprintFunctionLibrary|LoadJsonStringfromFile (Utilities|String|Append (Utilities|String|Append (Class|KismetSystemLibrary|GetProjectContentDirectory) "Charts/" (Variables|inGame|Datas|GetSongName) "/") "meta.json")))
  (bind _outstring (Class|IJsonObject|TryGetStringField _ijsonobject "Name"))
  (bind _outstring_2 (Class|IJsonObject|TryGetStringField _ijsonobject "MusicFile"))
  (bind _outstring_3 (Class|IJsonObject|TryGetStringField _ijsonobject "IllustrationFile"))
  (bind _outstring_4 (Class|IJsonObject|TryGetStringField _ijsonobject "Artist"))
  (bind _outstring_5 (Class|IJsonObject|TryGetStringField _ijsonobject "Illustrator"))
  (bind _outnumber (Class|IJsonObject|TryGetNumberField _ijsonobject "ChartOffset"))
  (Variables|inGame|Datas|SetSongInfo (Utilities|Struct|MakeS_SongInfo _outstring _outstring_2 _outstring_3 _outstring_4 _outstring_5 _outnumber))
  (bind _outarray (Class|IJsonObject|TryGetJsonObjectArrayField _ijsonobject "Difficulties"))
  (for _array_element _outarray
    (bind _outstring_6 (Class|IJsonObject|TryGetStringField _array_element "DifficultyName"))
    (bind _outnumber_2 (Class|IJsonObject|TryGetNumberField _array_element "Difficulty"))
    (bind _outstring_7 (Class|IJsonObject|TryGetStringField _array_element "Chart"))
    (bind _outstring_8 (Class|IJsonObject|TryGetStringField _array_element "ChartDesigner"))
    (Utilities|Array|Add (Variables|inGame|Datas|GetSongDifficultyLIst) (Utilities|Struct|MakeS_SongDifficultyInfo _outstring_6 (Math|Float|Truncate _outnumber_2) _outstring_7 _outstring_8)))
  (Utilities|Array|RemoveIndex (Variables|inGame|Datas|GetSongDifficultyLIst)))