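; SceneRenderAgent sets the scene background to the current song's illustration, loaded from disk at runtime.
; On BeginPlay it gets the game instance and builds the illustration path under the content directory's Charts folder from the song name and song info.
; The image is imported as a Texture2D into a dynamic material instance on the Background component.
; If the file is missing, it prints a warning and zeroes the material's opacity parameter.
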(event EventBeginPlay
  (bind _gi (CallFunction|GFuncGetGI))
  (Variables|Default|SetGI _gi)
  (CallFunction|Func#SetMaterial#))

(fn ConstructionScript)

(fn Func#FindIllustrationFile#
  (bind _returnvalue (Class|KismetSystemLibrary|GetProjectContentDirectory))
  (bind _gi (Variables|Default|GetGI))
  (bind _songinfo (Variables|/Game/BluePrints/MUNECK_GI.MUNECK_GI_C|GetSongInfo _gi))
  (bind _songname (Variables|/Game/BluePrints/MUNECK_GI.MUNECK_GI_C|GetSongName _gi))
  (bind _illustrationfile (Utilities|Struct|BreakS_SongInfo _songinfo))
  (bind _returnvalue_2 (Utilities|String|Append _returnvalue "Charts/" _songname "/" _illustrationfile))
  (if (Class|BlueprintPathsLibrary|FileExists _returnvalue_2)
    (return _returnvalue_2)
    (else
      ;[1 1 1] a back-up file needed FIXME
      (return "FileNotExistError"))))

(fn Func#SetMaterial#
  (bind _returnvalue (Rendering|Material|CreateDynamicMaterialInstance (Variables|Default|GetBackground) 0 "/Game/Textures/M_runtimeLoadMat.M_runtimeLoadMat" "None" :!class /Script/Engine.PrimitiveComponent))
  (bind _path (CallFunction|Func#FindIllustrationFile#))
  (if (Utilities|Enum|Equal(Enum) _path "FileNotExistError")
    (Development|PrintString "Background file not found, use default!" true true "(R=1.000000,G=0.388870,B=0.690603,A=1.000000)" 5.0)
    (Rendering|Material|SetScalarParameterValueonMaterials (Variables|Default|GetBackground) "opac" 0.0)
    (else
      (bind _returnvalue_2 (Class|KismetRenderingLibrary|ImportFileasTexture2D _path))
      (Rendering|Material|SetTextureParameterValue _returnvalue (Variables|Default|GettexParamName) _returnvalue_2))))