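; Base note actor for a rail-based, rhythm-style game, initialized from spawn info and moved at constant velocity from start toward a receiver target.
; Once progress reaches the target, distance moved while the receiver is active accumulates as a performance fraction of the note's length.
; When the note has fully passed or the receiver is inactive, it dispatches type, rail, length and performance for scoring.
; GameStateManager events pause and resume its tick logic or destroy it at game end.
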(event Custom|PauseGame
  ;[1 1 1] responding to GSM
  (Variables|Default|SetTick%20Enable false))

(event Custom|ResumeGame
  ;[1 1 1] responding to GSM
  (Variables|Default|SetTick%20Enable true))

(event Custom|LifeEnds
  (params (Reset%20Game :type Boolean))
  ;[1 1 1] responding to GSM
  (Actor|DestroyActor))

(event EventBeginPlay
  ;[1 1 1] responding to GSM
  (bind _returnvalue (Actor|GetActorOfClass "/Game/BluePrints/CoreGameplay/BP_GameStateManager.BP_GameStateManager_C"))
  (EventDispatchers|AssignEDGamePause _returnvalue (delegate Custom|PauseGame))
  (EventDispatchers|AssignEDGameResume _returnvalue (delegate Custom|ResumeGame))
  (EventDispatchers|AssignEDGameEnd _returnvalue (delegate Custom|LifeEnds)))

(event EventTick
  (params (DeltaSeconds :type Float%20%28single-precision%29))
  (if (Variables|Default|GetTick%20Enable)
    (bind _output_get (Variables|UpdateOnTick|SetDelta%20Speed (* (Variables|Default|GetSpeed%20of%20node) DeltaSeconds)))
    (CallFunction|Func#movement# _output_get)
    (if (Variables|UpdateOnTick|GetLife%20Ends)
      (Utilities|FlowControl|DoOnce false
        (:Completed
          (Development|PrintString "Node Life Ends")))
      (else
        (bind _touching_receiver (varupdates|Func#ProgressUpdate#))
        (if _touching_receiver
          (varupdates|Func#performanceUpdate# (Variables|UpdateOnTick|GetDelta%20Speed))
          ;[1 1 1] dispatch ED when ness
          ;;[1 1 1] life ends means all of self meshes pass the receiver
          (bind _lifeends (Overridables&Private(Self-useOnly)|Func#LifeEndStatusCheck#))
          (if _lifeends
            ;;[1 1 1] if LifeEnds is True, call ED(if True before, this function won't be called)
            (Variables|UpdateOnTick|SetLife%20Ends true)
            (Default|CallEDNodeGetScore (Utilities|Struct|MakeS_CNoteInfo (Variables|attributes|GetNode%20Type) (Variables|Attributes|GetRail) (Variables|Attributes|GetTime%20Length) (Variables|updateontick|Getperformance)))))))))

(fn ConstructionScript)

(fn Func#InitNode#
  (params (SpawnInfo :type S%20Note%20Spawn%20Info%20Structure))
  ;[1 1 1] placer will call on this.
  (bind _output_get (Variables|Attributes|SetSelfInfo SpawnInfo))
  (|BreakandSavetovariables _output_get)
  (Variables|Attributes|SetSpaceLength (* (Math|Vector|VectorLength (Variables|Attributes|GetSpeed%20Of%20Node)) (Variables|Attributes|GetTime%20Length))))

(fn Func#LifeEndStatusCheck#
  (return (or (> (Math|Vector|VectorLength (- (Variables|Attributes|GetTarget%20Pos) (Transformation|GetActorLocation))) (Variables|Attributes|GetSpaceLength)) (Math|Boolean|Equal(Boolean) (Variables|UpdateonTick|GetReceiver%20Status) false))))

(fn Func#PerformanceAddingRule#
  (params (moved%20distance :type Float%20%28single-precision%29))
  (return (/ moved%20distance (Variables|Attributes|GetSpaceLength))))

(fn Func#NodeonReceiver#
  (params (Receiver%20Status :type Boolean))
  (Variables|UpdateonTick|SetReceiver%20Status Receiver%20Status))

(fn Func#performanceUpdate#
  (params (deltaSpeed :type Vector))
  (if (Variables|UpdateonTick|GetReceiver%20Status)
    (bind _added_performance (Overridables&Private(Self-useOnly)|Func#PerformanceAddingRule# (Math|Vector|VectorLength deltaSpeed)))
    (Utilities|MAddPerformance _added_performance)))

(fn Func#ProgressUpdate#
  ;[1 1 1] save self loc as local var
  (LocalVariables|SetSelfLocation%28local%29 (Transformation|GetActorLocation))
  ;[1 1 1] update progress
  (if (>= (Variables|UpdateOnTick|GetProgress) 1.0)
    (return true)
    (else
      (|setprogresswithnewvalue)
      (return false))))

(fn Func#movement#
  (params (deltaSpeed :type Vector))
  (bind _returnvalue (Transformation|SetActorLocation (+ deltaSpeed (Transformation|GetActorLocation)) false false))
  (if _returnvalue
    (return)
    (else
      (Development|PrintString "BaseNOdeMovementError"))))