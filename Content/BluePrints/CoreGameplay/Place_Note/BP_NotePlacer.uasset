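; BP_NotePlacer is an actor that places rhythm notes in the level, following the game state's lifecycle.
; On BeginPlay it binds to BP_GameStateManager dispatchers, activating or deactivating its node placer component on start, pause and resume, and destroying itself at game end.
; When note dropping starts, it initializes that component with level variables and forwards PlaceNode signals from Notes_controller actors for spawning.
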(event Custom|LifeBegin
  ;[1 1 1] init components
  (Components|Activation|Activate (Variables|Default|GetBPAC_NodePlacerComponent) false)
  (Default|Func#initLevelVariableComponent# (Variables|Default|GetBPAC_NodePlacerComponent) (Variables|Default|GetLevelVariablesComponent))
  ;[1 1 1] bind place node signal from note controller
  (bind _outactors (Actor|GetAllActorsOfClass "/Game/BluePrints/CoreGameplay/Notes_controller.Notes_controller_C"))
  (EventDispatchers|AssignEDPlaceNode _outactors (delegate Custom|PlaceNode)))

(event Custom|PlaceNode
  (params (SpawnNodeInfo :type S%20Note%20Info%20Structure))
  ;[1 1 1] bind place node signal from note controller
  (Default|Func#placeNodeandInit# (Variables|Default|GetBPAC_NodePlacerComponent) SpawnNodeInfo))

(event Custom|GamePause
  (Components|Activation|Deactivate (Variables|Default|GetBPAC_NodePlacerComponent)))

(event Custom|GameResume
  (Components|Activation|Activate (Variables|Default|GetBPAC_NodePlacerComponent) false))

(event Custom|LifeEnds
  (params (Is%20Game%20End :type Boolean))
  (Actor|DestroyActor))

(event EventBeginPlay
  (bind _returnvalue (Actor|GetActorOfClass "/Game/BluePrints/CoreGameplay/BP_GameStateManager.BP_GameStateManager_C"))
  (EventDispatchers|BindEventtoEDNoteStartDropping _returnvalue (delegate Custom|LifeBegin))
  (EventDispatchers|AssignEDGamePause _returnvalue (delegate Custom|GamePause))
  (EventDispatchers|AssignEDGameResume _returnvalue (delegate Custom|GameResume))
  (EventDispatchers|AssignEDGameEnd _returnvalue (delegate Custom|LifeEnds)))

(fn ConstructionScript)