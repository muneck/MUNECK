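; BP_NoteAvoid is the avoid-type note, a child note Blueprint that overrides initialization, life-end and scoring.
; BeginPlay selects the avoid body material, calls CreateMesh and applies the dynamic material to the body.
; Init adds a static mesh stretched along X to match SpaceLength, offset by half its length.
; Performance above a small threshold ends its life early, and it scores only while Performance stays below that threshold.
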(event EventBeginPlay
  (|CallParentFunction)
  (Variables|Default|SetBodyMaterial "/Game/Materials/CoreGamePlay/Notes/MI_NoteAvoidBodyMaterial.MI_NoteAvoidBodyMaterial")
  (CallFunction|CreateMesh)
  (Rendering|Material|SetMaterial (Variables|Default|GetBodyMesh) 0 (Variables|Default|GetBody_DMI)))

(fn ConstructionScript)

(fn Func#InitNode#
  (params (SpawnInfo :type S%20Note%20Spawn%20Info%20Structure))
  (|CallParentFunction SpawnInfo)
  (bind _tailtransform (CallFunction|Func#CalculateTransform#))
  (AddComponent|AddStaticMeshComponent false _tailtransform))

(fn Func#CalculateTransform#
  (bind _spacelength (Variables|Default|GetSpaceLength))
  (bind _output_get (Variables|Default|SetTailTransform (Math|Transform|MakeTransform (Math|Vector|MakeVector (/ _spacelength 2.0) 0.0 0.0) "0, 0, 0" (Math|Vector|MakeVector (/ _spacelength 1e+02) 0.12 1.0))))
  (return _output_get))

(fn Func#LifeEndStatusCheck#
  (bind _lifeends (|CallParentFunction))
  (return (or _lifeends (> (Variables|Default|Getperformance) 0.05))))

(fn Func#GetScoring#
  (return (< (Variables|Default|Getperformance) 0.05)))