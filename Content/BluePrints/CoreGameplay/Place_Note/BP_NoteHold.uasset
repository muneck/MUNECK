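; Hold note for what appears to be a rhythm game, extending a parent note with a stretched body and a tail.
; On node init it adds body and tail static mesh components, placing both and scaling the body from SpaceLength.
; BeginPlay assigns the hold material, creates the mesh and applies BodyDMI to the head.
; Its life-end check also passes when ReceiverStatus is false, alongside the parent's condition.
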(event EventBeginPlay
  (|CallParentFunction)
  (Variables|Default|SetHeadMaterial "/Game/Materials/CoreGamePlay/Notes/MI_NoteHoldBodyMaterial.MI_NoteHoldBodyMaterial")
  (CallFunction|CreateMesh)
  (Rendering|Material|SetMaterial (Variables|Default|GetHeadMesh) 0 (Variables|Default|GetBody_DMI)))

(fn ConstructionScript)

(fn Func#InitNode#
  (params (SpawnInfo :type S%20Note%20Spawn%20Info%20Structure))
  (|CallParentFunction SpawnInfo)
  (CallFunction|AddBodyMesh))

(fn Func#CalculateTransform#
  (bind _returnvalue (+ 24.5 27.700001))
  (bind _spacelength (Variables|Default|GetSpaceLength))
  (bind _returnvalue_2 (/ _spacelength _returnvalue))
  (bind _output_get (Variables|Default|SetBodyTransform (Math|Transform|MakeTransform (Math|Vector|MakeVector (* _returnvalue_2 27.700001) 0.0 2.2e+02) "0,90.000000, 0" (Math|Vector|MakeVector 1.0 _returnvalue_2 1.0))))
  (return _output_get (Math|Transform|MakeTransform (Math|Vector|MakeVector (+ (Variables|Default|GetSpaceLength) 1e+01) 0.0 2.1e+02) "0,90.000000, 0")))

(fn Func#LifeEndStatusCheck#
  ;[1 1 1] pass receiver
  (bind _lifeends (|CallParentFunction))
  (return (or _lifeends (Math|Boolean|Equal(Boolean) (Variables|Default|GetReceiver%20Status) false))))

(fn AddBodyMesh
  (bind (_bodytransform _tailtransform) (CallFunction|Func#CalculateTransform#))
  (bind _returnvalue (AddComponent|AddStaticMeshComponent false _bodytransform))
  (Rendering|Material|SetMaterial _returnvalue 0 "/Game/Materials/CoreGamePlay/Notes/M_NoteHold_Body.M_NoteHold_Body")
  (bind _returnvalue_2 (AddComponent|AddStaticMeshComponent false _tailtransform))
  (Rendering|Material|SetMaterial _returnvalue_2 0 "/Game/Materials/CoreGamePlay/Notes/M_NoteHoldTail.M_NoteHoldTail"))