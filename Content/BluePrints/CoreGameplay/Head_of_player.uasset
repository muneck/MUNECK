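; Head_of_player is an actor that turns face-capture data into the player's head rotation.
; On BeginPlay it binds to the GameStateManager's start, pause, resume and end events, which start the pipeline, toggle its work flag, or stop it and destroy the actor.
; While working, Tick stores the first face's status as HeadRotation.
; The head-bump detection function is a stub that always returns false.
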(event Custom|GameStart
  (CallFunction|StartPipeline))

(event Custom|LifeEnds
  (params (Reset%20Game :type Boolean))
  (CallFunction|StopPipeline)
  (Actor|DestroyActor))

(event Custom|PausePipeline
  (Variables|Default|SetIn%20Work false))

(event Custom|ResumePipeline
  (Variables|Default|SetIn%20Work true))

(event EventBeginPlay
  (bind _returnvalue (Actor|GetActorOfClass "/Game/BluePrints/CoreGameplay/BP_GameStateManager.BP_GameStateManager_C"))
  (EventDispatchers|AssignEDGameStart _returnvalue (delegate Custom|GameStart))
  (EventDispatchers|AssignEDGamePause _returnvalue (delegate Custom|PausePipeline))
  (EventDispatchers|AssignEDGameResume _returnvalue (delegate Custom|ResumePipeline))
  (EventDispatchers|AssignEDGameEnd _returnvalue (delegate Custom|LifeEnds)))

(event EventTick
  (params (DeltaSeconds :type Float%20%28single-precision%29))
  (if (Variables|Default|GetIn%20Work)
    (Variables|Default|SetHead%20Rotation (Class|MediaPipeLandmarkObserverComponent|GetFaceStatus (Variables|Default|GetFace)))))

(fn ConstructionScript)

(fn Fuc#HeadBumpDetect
  (params (collision%20component :type Static%20Mesh%20Component%20Object%20Reference) (Collide%20Node :type Actor%20Object%20Reference))
  (return false))