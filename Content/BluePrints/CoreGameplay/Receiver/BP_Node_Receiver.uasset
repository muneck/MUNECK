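; BP_Node_Receiver is a note receiver that activates when the player's head turn, tilt or nod falls within its configured ranges.
; Each tick it reads Head_of_player's rotation and swaps its material to show the state.
; While active, it destroys overlapping Note_flick actors and fires GetPoint for each.
; Also every tick, unless its ID is -999, it saves its transform, ID and angle ranges to a per-ID SaveGame slot.
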(event EventTick
  (params (DeltaSeconds :type Float%20%28single-precision%29))
  (bind _main_bodymesh (Variables|Default|Getmain_bodymesh))
  (Utilities|FlowControl|Sequence
    (:then_0
      (bind _is_activated (CallFunction|Fuc#IsActivated#))
      ;[1 1 1] set material according to status
      (if _is_activated
        (Rendering|Material|SetMaterial _main_bodymesh 0 "/Game/BluePrints/CoreGameplay/Materials/M_Excited_Receiver.M_Excited_Receiver")
        (for _array_element (Collision|GetOverlappingActors "/Game/BluePrints/CoreGameplay/Note_flick.Note_flick_C" :!class /Script/Engine.Actor)
          (bind _asnote_flick (Utilities|Casting|CastToNote_flick _array_element))
          (Actor|DestroyActor _asnote_flick)
          (Default|CallGetPoint _asnote_flick))
        (else
          (Rendering|Material|SetMaterial _main_bodymesh 0 "/Engine/BasicShapes/BasicShapeMaterial.BasicShapeMaterial"))))
    (:then_1
      (CallFunction|Func#saveStructifNeeded#))))

(fn ConstructionScript)

(fn Fuc#IsActivated#
  (bind _outactors (Actor|GetAllActorsOfClass "/Game/BluePrints/CoreGameplay/Head_of_player.Head_of_player_C"))
  (bind _ashead_of_player (Utilities|Casting|CastToHead_of_player (Utilities|Array|Get(acopy) _outactors)))
  (bind _output_get (Variables|Default|SetStatus (Math|Boolean|ORBoolean (Utilities|MIsValueinRange (Variables|Default|GetTurnAngleRange) (.Turn (Utilities|Struct|BreakMediaPipeFaceRotation (Variables|/Game/BluePrints/CoreGameplay/Head_of_player.Head_of_player_C|GetHead%20Rotation _ashead_of_player)))) (Utilities|MIsValueinRange (Variables|Default|GetTiltAngleRange) (.Tilt (Utilities|Struct|BreakMediaPipeFaceRotation (Variables|/Game/BluePrints/CoreGameplay/Head_of_player.Head_of_player_C|GetHead%20Rotation _ashead_of_player)))) (Utilities|MIsValueinRange (Variables|Default|GetNodAngleRange) (.Nod (Utilities|Struct|BreakMediaPipeFaceRotation (Variables|/Game/BluePrints/CoreGameplay/Head_of_player.Head_of_player_C|GetHead%20Rotation _ashead_of_player)))))))
  (return _output_get))

(fn InitStruct
  (Variables|Default|SetAdvance%20Receiver%20Struct (Utilities|Struct|MakeS_receiverInfoAdvance (Transformation|GetActorTransform) (Variables|Default|GetID) (Variables|Default|GetTiltAngleRange) (Variables|Default|GetTurnAngleRange) (Variables|Default|GetNodAngleRange)))
  (Variables|Default|SetReceiver%20Struct ""))

(fn Func#saveStructifNeeded#
  (if (!= (Variables|Default|GetID) -999)
    (bind _output_get (Variables|Default|SetSlot (Utilities|String|Append "ADVreceiver" (Utilities|String|ToString(Integer) (Variables|Default|GetID)))))
    (CallFunction|InitStruct)
    (bind _returnvalue (SaveGame|DoesSaveGameExist _output_get))
    (if _returnvalue
      (bind _returnvalue_2 (SaveGame|LoadGamefromSlot (Variables|Default|GetSlot)))
      (bind _assg_advance_receiver_init (Utilities|Casting|CastToSG_AdvanceReceiverInit _returnvalue_2))
      (Variables|Default|SetSaveGameObj _assg_advance_receiver_init)
      (else
        (bind _returnvalue_3 (SaveGame|CreateSaveGameObject "/Game/BluePrints/CoreGameplay/Receiver/SG_AdvanceReceiverInit.SG_AdvanceReceiverInit_C"))
        (Variables|Default|SetSaveGameObj _returnvalue_3)))
    (Variables|/Game/BluePrints/CoreGameplay/Receiver/SG_AdvanceReceiverInit.SG_AdvanceReceiverInit_C|SetAdvanceReceiverStruct%28SavegameVar%29 (Variables|Default|GetSaveGameObj) (Variables|Default|GetAdvance%20Receiver%20Struct))
    (bind _returnvalue_4 (SaveGame|SaveGametoSlot (Variables|Default|GetSaveGameObj) (Variables|Default|GetSlot)))
    (if _returnvalue_4
      (Variables|Default|SetSavedStatus true)
      (else
        (Variables|Default|SetSavedStatus false)))
    (else
      (Development|PrintString "Receiver Saving End, variables are null"))))