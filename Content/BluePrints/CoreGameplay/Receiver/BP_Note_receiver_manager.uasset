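; Manager actor that spawns the note receivers when the game starts and destroys itself when the game ends, via BP_GameStateManager dispatchers.
; For each listed ID, it looks up receiver data in the GameInstance and spawns a BP_Note_Receiver with its ID and angle ranges.
; Location comes from the viewport-scaled rail end position, while rotation and scale come from the stored struct.
; An older save-slot loading path remains disconnected.
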(event Custom|ED_GameStart
  ;[1 1 1] Load receivers from ADVreceiver{ID}.sav
  (for _array_element (Variables|Default|GetID_List)
    (if (.ReturnValue (Utilities|Map|Find (Variables|/Game/BluePrints/MUNECK_GI.MUNECK_GI_C|GetReceiverInfo (Variables|Default|GetGI)) _array_element))
      (CallFunction|Func#SpawnandLoadAdvanceStructIntoReceiver# (.Value (Utilities|Map|Find (Variables|/Game/BluePrints/MUNECK_GI.MUNECK_GI_C|GetReceiverInfo (Variables|Default|GetGI)) _array_element)))
      (else
        (Development|PrintString "Hello")))))

(event Custom|LifeEnds
  (params (Reset%20Game :type Boolean))
  (Actor|DestroyActor))

(event EventBeginPlay
  (bind _gi (CallFunction|GFuncGetGI))
  (Variables|Default|SetGI _gi)
  (bind _returnvalue (Actor|GetActorOfClass "/Game/BluePrints/CoreGameplay/BP_GameStateManager.BP_GameStateManager_C"))
  (EventDispatchers|AssignEDGameStart _returnvalue (delegate Custom|ED_GameStart))
  (EventDispatchers|AssignEDGameEnd _returnvalue (delegate Custom|LifeEnds)))

(fn ConstructionScript)

(fn Func#SpawnandLoadAdvanceStructIntoReceiver#
  (params (Struct :type S%20Receiver%20Info%20Advance%20Structure))
  (bind (_absolutetransform _id _tiltanglerange _turnanglerange _nodanglerange) (Utilities|Struct|BreakS_receiverInfoAdvance Struct))
  (bind (_location _rotation _scale) (Math|Transform|BreakTransform _absolutetransform))
  (bind _v_in_levels (CallFunction|VportScaled2map (.Value (Utilities|Map|Find (Variables|/Game/BluePrints/MUNECK_GI.MUNECK_GI_C|GetRail_EndPos (Variables|Default|GetGI)) _id))))
  (bind _returnvalue (Game|SpawnActorfromClass "/Game/BluePrints/CoreGameplay/Receiver/BP_Note_Receiver.BP_Note_Receiver_C" (Math|Transform|MakeTransform _v_in_levels _rotation _scale) "AlwaysSpawn" 0 0))
  (Variables|/Game/BluePrints/CoreGameplay/Receiver/BP_Note_Receiver.BP_Note_Receiver_C|SetID _returnvalue _id)
  (Variables|/Game/BluePrints/CoreGameplay/Receiver/BP_Note_Receiver.BP_Note_Receiver_C|SetTurnAngleRange _returnvalue _turnanglerange)
  (Variables|/Game/BluePrints/CoreGameplay/Receiver/BP_Note_Receiver.BP_Note_Receiver_C|SetNodAngleRange _returnvalue _nodanglerange)
  (Variables|/Game/BluePrints/CoreGameplay/Receiver/BP_Note_Receiver.BP_Note_Receiver_C|SetTiltAngleRange _returnvalue _tiltanglerange))