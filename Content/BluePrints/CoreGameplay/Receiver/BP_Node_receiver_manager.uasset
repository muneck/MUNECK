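; Manager that rebuilds the level's BP_Node_Receiver actors from save games on BeginPlay.
; For each ID in IDList it loads an "ADVreceiver"-prefixed slot and spawns a receiver at the saved transform with its ID and turn, nod and tilt ranges.
; A failed cast prints a loading error.
; An unconnected variant for plain "receiver" saves, which does not restore nod range, remains in the graph.
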(event EventBeginPlay
  (for _array_element (Variables|Default|GetID_List)
    (bind _returnvalue (SaveGame|LoadGamefromSlot (Utilities|String|Append "ADVreceiver" (Utilities|String|ToString(Integer) _array_element))))
    (bind _assg_advance_receiver_init (Utilities|Casting|CastToSG_AdvanceReceiverInit _returnvalue)
      (:then
        (CallFunction|Func#loadAdvanceStructIntoReceiver# (Variables|/Game/BluePrints/CoreGameplay/Receiver/SG_AdvanceReceiverInit.SG_AdvanceReceiverInit_C|GetAdvanceReceiverStruct%28SavegameVar%29 _assg_advance_receiver_init)))
      (:CastFailed
        (Utilities|MRaiseError "Loading"))))
  (Development|PrintString "Receiver Load Complete"))

(fn ConstructionScript)

(fn Func#loadStructIntoReceiver#
  (params (Struct :type S%20Receiver%20Info%20Structure))
  (bind (_absolutetransform _id _tiltanglerange _turnanglerange) (Utilities|Struct|BreakS_receiverInfo Struct))
  (bind _returnvalue (Game|SpawnActorfromClass "/Game/BluePrints/CoreGameplay/Receiver/BP_Node_Receiver.BP_Node_Receiver_C" _absolutetransform "AlwaysSpawn" 0 0))
  (Variables|/Game/BluePrints/CoreGameplay/Receiver/BP_Node_Receiver.BP_Node_Receiver_C|SetID _returnvalue _id)
  (Variables|/Game/BluePrints/CoreGameplay/Receiver/BP_Node_Receiver.BP_Node_Receiver_C|SetTurnAngleRange _returnvalue _turnanglerange)
  (Variables|/Game/BluePrints/CoreGameplay/Receiver/BP_Node_Receiver.BP_Node_Receiver_C|SetNodAngleRange _returnvalue "")
  (Variables|/Game/BluePrints/CoreGameplay/Receiver/BP_Node_Receiver.BP_Node_Receiver_C|SetTiltAngleRange _returnvalue _tiltanglerange))

(fn Func#loadAdvanceStructIntoReceiver#
  (params (Struct :type S%20Receiver%20Info%20Advance%20Structure))
  (bind (_absolutetransform _id _tiltanglerange _turnanglerange _nodanglerange) (Utilities|Struct|BreakS_receiverInfoAdvance Struct))
  (bind _returnvalue (Game|SpawnActorfromClass "/Game/BluePrints/CoreGameplay/Receiver/BP_Node_Receiver.BP_Node_Receiver_C" _absolutetransform "AlwaysSpawn" 0 0))
  (Variables|/Game/BluePrints/CoreGameplay/Receiver/BP_Node_Receiver.BP_Node_Receiver_C|SetID _returnvalue _id)
  (Variables|/Game/BluePrints/CoreGameplay/Receiver/BP_Node_Receiver.BP_Node_Receiver_C|SetTurnAngleRange _returnvalue _turnanglerange)
  (Variables|/Game/BluePrints/CoreGameplay/Receiver/BP_Node_Receiver.BP_Node_Receiver_C|SetNodAngleRange _returnvalue _nodanglerange)
  (Variables|/Game/BluePrints/CoreGameplay/Receiver/BP_Node_Receiver.BP_Node_Receiver_C|SetTiltAngleRange _returnvalue _tiltanglerange))