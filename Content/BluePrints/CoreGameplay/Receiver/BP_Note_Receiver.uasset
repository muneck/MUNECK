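; BP_Note_Receiver is a receiver actor that activates from the player's head rotation and signals overlapping note actors.
; Each Tick it saves its transform, ID and angle ranges to an ID-named save slot, unless the ID is unset.
; It is active when the Head_of_player's turn, tilt or nod falls within its range.
; That status swaps the body material and is passed to every overlapping BP_NoteBaseActor.
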(event EventTick
  (params (DeltaSeconds :type Float%20%28single-precision%29))
  (Utilities|MMainSequence
    (:SavegameLogic
      (CallFunction|Func#save/updateStruct#))
    (:ActivationStatusUpdate
      (bind _is_activated (CallFunction|Fuc#IsActivated#))
      (CallFunction|Func#updateAppearance# _is_activated))
    (:Interact%20with%20Nodes
      (for _array_element (Collision|GetOverlappingActors "/Game/BluePrints/CoreGameplay/Place_Note/BP_NoteBaseActor.BP_NoteBaseActor_C" :!class /Script/Engine.Actor)
        (bind _asbp_note_base_actor (Utilities|Casting|CastToBP_NoteBaseActor _array_element))
        (Default|Func#NodeonReceiver# _asbp_note_base_actor (Variables|Default|GetSelfActivationStatus))))))

(fn ConstructionScript)

(fn Fuc#IsActivated#
  (bind _outactors (Actor|GetAllActorsOfClass "/Game/BluePrints/CoreGameplay/Head_of_player.Head_of_player_C"))
  (bind _ashead_of_player (Utilities|Casting|CastToHead_of_player (Utilities|Array|Get(acopy) _outactors)))
  (bind _output_get (Variables|Default|SetSelfActivationStatus (Math|Boolean|ORBoolean (Utilities|MIsValueinRange (Variables|Default|GetTurnAngleRange) (.Turn (Utilities|Struct|BreakMediaPipeFaceRotation (Variables|/Game/BluePrints/CoreGameplay/Head_of_player.Head_of_player_C|GetHead%20Rotation _ashead_of_player)))) (Utilities|MIsValueinRange (Variables|Default|GetTiltAngleRange) (.Tilt (Utilities|Struct|BreakMediaPipeFaceRotation (Variables|/Game/BluePrints/CoreGameplay/Head_of_player.Head_of_player_C|GetHead%20Rotation _ashead_of_player)))) (Utilities|MIsValueinRange (Variables|Default|GetNodAngleRange) (.Nod (Utilities|Struct|BreakMediaPipeFaceRotation (Variables|/Game/BluePrints/CoreGameplay/Head_of_player.Head_of_player_C|GetHead%20Rotation _ashead_of_player)))))))
  (return _output_get))

(fn Func#InitADVStruct#
  (Variables|Default|SetAdvance%20Receiver%20Struct (Utilities|Struct|MakeS_receiverInfoAdvance (Transformation|GetActorTransform) (Variables|Default|GetID) (Variables|Default|GetTiltAngleRange) (Variables|Default|GetTurnAngleRange) (Variables|Default|GetNodAngleRange))))

(fn Func#save/updateStruct#
  ;[1 1 1] If parameters are set
  (if (!= (Variables|Default|GetID) -999)
    (bind _output_get (Variables|Default|SetSlot (Utilities|String|Append "ADVreceiver" (Utilities|String|ToString(Integer) (Variables|Default|GetID)))))
    (CallFunction|Func#InitADVStruct#)
    (bind _returnvalue (SaveGame|DoesSaveGameExist _output_get))
    (if _returnvalue
      (bind _returnvalue_2 (SaveGame|LoadGamefromSlot (Variables|Default|GetSlot)))
      (bind _assg_advance_receiver_init (Utilities|Casting|CastToSG_AdvanceReceiverInit _returnvalue_2))
      (Variables|Default|SetSaveGameObj _assg_advance_receiver_init)
      (else
        (bind _returnvalue_3 (SaveGame|CreateSaveGameObject "/Game/BluePrints/CoreGameplay/Receiver/SG_AdvanceReceiverInit.SG_AdvanceReceiverInit_C"))
        (Variables|Default|SetSaveGameObj _returnvalue_3)))
    (Variables|/Game/BluePrints/CoreGameplay/Receiver/SG_AdvanceReceiverInit.SG_AdvanceReceiverInit_C|SetAdvanceReceiverStruct%28SavegameVar%29 (Variables|Default|GetSaveGameObj) (Variables|Default|GetAdvance%20Receiver%20Struct))
    (bind _returnvalue_4 (SaveGame|SaveGametoSlot (Variables|Default|GetSaveGameObj) (Variables|Default|GetSlot)))
    (Utilities|MUpdateSaveStatus _returnvalue_4)
    (else
      (Development|PrintString "Receiver Saving End, variables are null"))))

(fn Func#updateAppearance#
  (params (Condition :type Boolean))
  (bind _main_bodymesh (Variables|Default|Getmain_bodymesh))
  ;[1 1 1] set material according to status
  (if Condition
    (Rendering|Material|SetMaterial _main_bodymesh 0 "/Game/BluePrints/CoreGameplay/Materials/M_Excited_Receiver.M_Excited_Receiver")
    (else
      (Rendering|Material|SetMaterial _main_bodymesh 0 "/Engine/BasicShapes/BasicShapeMaterial.BasicShapeMaterial"))))