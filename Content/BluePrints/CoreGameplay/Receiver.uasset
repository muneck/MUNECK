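; Receiver actor that collects Note_flick notes when the player's head rotation activates it, in what appears to be a rhythm-style game.
; Each Tick it finds Head_of_player and counts as active if Turn, Tilt or Nod falls within its configured angle range.
; While active it shows an excited material, destroys overlapping notes and calls GetPoint for each; otherwise it shows the basic material.
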(event EventBeginPlay)

(event Collision|EventActorBeginOverlap
  (params (OtherActor :type Actor%20Object%20Reference)))

(event EventTick
  (params (DeltaSeconds :type Float%20%28single-precision%29))
  (bind _main_bodymesh (Variables|Default|Getmain_bodymesh))
  (Utilities|FlowControl|Sequence
    (:then_0
      (bind _is_activated (CallFunction|Fuc#IsActivated#))
      ;[1 1 1] set material according to status
      (if _is_activated
        (Rendering|Material|SetMaterial _main_bodymesh 0 "/Game/BluePrints/CoreGameplay/Materials/M_Excited_Receiver.M_Excited_Receiver")
        (for _array_element (Collision|GetOverlappingActors "/Game/BluePrints/CoreGameplay/Note_flick.Note_flick_C" :!class /Script/Engine.Actor)
          (bind _asnote_flick (Utilities|Casting|CastToNote_flick _array_element))
          (Actor|DestroyActor _asnote_flick)
          (Default|CallGetPoint _asnote_flick))
        (else
          (Rendering|Material|SetMaterial _main_bodymesh 0 "/Engine/BasicShapes/BasicShapeMaterial.BasicShapeMaterial"))))))

(fn ConstructionScript)

(fn Fuc#IsActivated#
  (bind _outactors (Actor|GetAllActorsOfClass "/Game/BluePrints/CoreGameplay/Head_of_player.Head_of_player_C"))
  (bind _ashead_of_player (Utilities|Casting|CastToHead_of_player (Utilities|Array|Get(acopy) _outactors)))
  (bind _output_get (Variables|Default|SetStatus (Math|Boolean|ORBoolean (and (>= (Variables|Default|GetTurnAngleMax) (.Turn (Utilities|Struct|BreakMediaPipeFaceRotation (Variables|/Game/BluePrints/CoreGameplay/Head_of_player.Head_of_player_C|GetHead%20Rotation _ashead_of_player)))) (>= (.Turn (Utilities|Struct|BreakMediaPipeFaceRotation (Variables|/Game/BluePrints/CoreGameplay/Head_of_player.Head_of_player_C|GetHead%20Rotation _ashead_of_player))) (Variables|Default|GetTurnAngleMin))) (and (>= (Variables|Default|GetTiltAngleMax) (.Tilt (Utilities|Struct|BreakMediaPipeFaceRotation (Variables|/Game/BluePrints/CoreGameplay/Head_of_player.Head_of_player_C|GetHead%20Rotation _ashead_of_player)))) (>= (.Tilt (Utilities|Struct|BreakMediaPipeFaceRotation (Variables|/Game/BluePrints/CoreGameplay/Head_of_player.Head_of_player_C|GetHead%20Rotation _ashead_of_player))) (Variables|Default|GetTiltAngleMin))) (and (>= (Variables|Default|GetNodAngleMax) (.Nod (Utilities|Struct|BreakMediaPipeFaceRotation (Variables|/Game/BluePrints/CoreGameplay/Head_of_player.Head_of_player_C|GetHead%20Rotation _ashead_of_player)))) (>= (.Nod (Utilities|Struct|BreakMediaPipeFaceRotation (Variables|/Game/BluePrints/CoreGameplay/Head_of_player.Head_of_player_C|GetHead%20Rotation _ashead_of_player))) (Variables|Default|GetNodAngleMin))))))
  (return _output_get))