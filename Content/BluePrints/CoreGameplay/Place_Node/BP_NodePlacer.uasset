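; BP_NodePlacer spawns or places flick, hold and avoid notes on rails in what appears to be a rhythm game.
; On BeginPlay it initializes its placer component with the level variables and binds to the placement dispatchers of Notes_controller actors.
; Each handler has the component place a note by rail, delay and type, casts it, sets length for hold and avoid, then initializes it.
; Failed casts print an error.
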(event Custom|Place%20Flick
  (params (Rail :type Integer) (delay%20time :type Float%20%28single-precision%29))
  (bind _spawnednode (Default|Func#placeNoteonRoute# (Variables|Default|GetBPAC_NodePlacerComponent) Rail "NewEnumerator0" delay%20time))
  (bind _asbp_node_flick (Utilities|Casting|CastToBP_NodeFlick _spawnednode)
    (:then
      (Default|Func#InitNode# _asbp_node_flick))
    (:CastFailed
      (Utilities|MRaiseError))))

(event Custom|Place%20Hold
  (params (rail :type Integer) (Length :type Float%20%28single-precision%29) (delay%20time :type Float%20%28single-precision%29))
  (bind _spawnednode (Default|Func#placeNoteonRoute# (Variables|Default|GetBPAC_NodePlacerComponent) rail "NewEnumerator1" delay%20time))
  (bind _asbp_node_hold (Utilities|Casting|CastToBP_NodeHold _spawnednode)
    (:then
      (Variables|/Game/BluePrints/CoreGameplay/Place_Node/BP_NodeHold.BP_NodeHold_C|SetTimeLength _asbp_node_hold Length)
      (Default|Func#InitNode# _asbp_node_hold))
    (:CastFailed
      (Utilities|MRaiseError))))

(event Custom|Place%20Avoid
  (params (rail :type Integer) (Length :type Float%20%28single-precision%29) (delay%20time :type Float%20%28single-precision%29))
  (bind _spawnednode (Default|Func#placeNoteonRoute# (Variables|Default|GetBPAC_NodePlacerComponent) rail "NewEnumerator2" delay%20time))
  (bind _asbp_node_avoid (Utilities|Casting|CastToBP_NodeAvoid _spawnednode)
    (:then
      (Variables|/Game/BluePrints/CoreGameplay/Place_Node/BP_NodeAvoid.BP_NodeAvoid_C|SetTimeLength _asbp_node_avoid Length)
      (Default|Func#InitNode# _asbp_node_avoid))
    (:CastFailed
      (Utilities|MRaiseError))))

(event EventBeginPlay
  (Components|Activation|Activate (Variables|Default|GetBPAC_NodePlacerComponent) false)
  (Default|Func#initLevelVariableComponent# (Variables|Default|GetBPAC_NodePlacerComponent) (Variables|Default|GetLevelVariablesComponent))
  (bind _outactors (Actor|GetAllActorsOfClass "/Game/BluePrints/CoreGameplay/Notes_controller.Notes_controller_C"))
  (EventDispatchers|AssignEDPlaceFlick _outactors (delegate Custom|Place%20Flick))
  (EventDispatchers|AssignEDPlaceHold _outactors (delegate Custom|Place%20Hold))
  (EventDispatchers|AssignEDPlaceAvoid _outactors (delegate Custom|Place%20Avoid)))

(fn ConstructionScript)