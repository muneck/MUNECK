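; BP_NodeHold is a hold-type node whose length scales with its speed and hold duration, apparently for timed-input gameplay.
; Initialization adds a static mesh tail, offset by half and stretched along X to the length computed from BPAC_NodeComponent's speed times TimeLength.
; That length also drives performance (moved distance as a fraction, zero without ReceiverStatus) and life end, once distance past the receiver exceeds it.
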(event EventBeginPlay)

(event Collision|EventActorBeginOverlap
  (params (OtherActor :type Actor%20Object%20Reference)))

(event EventTick
  (params (DeltaSeconds :type Float%20%28single-precision%29)))

(fn ConstructionScript)

(fn Func#InitNode#
  (bind _tailtransform (CallFunction|Func#CalculateTransform#))
  (AddComponent|AddStaticMeshComponent false _tailtransform))

(fn Func#CalculateTransform#
  (bind _output_get (Variables|Default|SetSpaceLength (* (Math|Vector|VectorLength (Variables|/Game/BluePrints/CoreGameplay/Place_Node/BPAC_NodeComponent.BPAC_NodeComponent_C|GetSpeed%20of%20node (Actor|GetComponentbyClass "/Game/BluePrints/CoreGameplay/Place_Node/BPAC_NodeComponent.BPAC_NodeComponent_C"))) (Variables|Default|GetTimeLength))))
  (bind _output_get_2 (Variables|Default|SetTailTransform (Math|Transform|MakeTransform (Math|Vector|MakeVector (/ _output_get 2.0) 0.0 0.0) "0, 0, 0" (Math|Vector|MakeVector (/ _output_get 1e+02) 0.12 1.0))))
  (return _output_get_2))

(fn Func#updatePerformance#
  (params (moved%20distance :type Float%20%28single-precision%29))
  (if (Variables|Default|GetReceiver%20Status)
    (return (/ moved%20distance (Variables|Default|GetSpaceLength)))
    (else
      (return 0.0))))

(fn Func#LifeEndStatusCheck#
  (params (Distance%20passing%20receiver :type Float%20%28single-precision%29))
  (if (> Distance%20passing%20receiver (Variables|Default|GetSpaceLength))
    (return true)
    (else
      (return false))))