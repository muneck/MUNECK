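; BP_PlayingDataCollector is a gameplay data recorder meant to capture per-frame head rotation, score and completed nodes.
; BeginPlay caches the Head_of_player actor; while StartRecord is set, Tick refreshes values and packs them into CurrentFrameData as an SFrameData struct.
; The refresh function is a placeholder that zeroes score and rotation without reading the cached actor.
; An unconnected fragment notes a planned switch to a game state manager for score.
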(event EventBeginPlay
  (bind _returnvalue (Actor|GetActorOfClass "/Game/BluePrints/CoreGameplay/Head_of_player.Head_of_player_C"))
  (Variables|Actors|SetHead%20of%20Player _returnvalue))

(event EventTick
  (params (DeltaSeconds :type Float%20%28single-precision%29))
  (if (Variables|Default|GetStart_record)
    (CallFunction|Func#getSavingData#)
    (Variables|Default|SetCurrentFrameData (Utilities|Struct|MakeS_FrameData (Variables|Default|GetHead%20Rotation) (Variables|Default|GetCompleted%20Node%20List) (Variables|Default|GetCurrent%20Score)))))

(fn ConstructionScript)

(fn Func#getSavingData#
  (Variables|Default|SetCurrent%20Score 0.0)
  (Variables|Default|SetHead%20Rotation "0, 0, 0"))