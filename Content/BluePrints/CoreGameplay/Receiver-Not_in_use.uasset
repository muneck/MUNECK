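; Rhythm-style note receiver actor, named as not in use, that the player activates by head rotation.
; Each tick it checks whether Head_of_player's turn, tilt or nod falls within its angle ranges; any one suffices.
; While active it shows an excited material, destroys overlapping Note_flick actors and calls GetPoint for each.
; BeginPlay saves its transform, ID, tilt and turn ranges to a per-ID slot if none exists.
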(event Collision|EventActorBeginOverlap
  (params (OtherActor :type Actor%20Object%20Reference)))

(event EventTick
  (params (DeltaSeconds :type Float%20%28single-precision%29))
  (bind _main_bodymesh (Variables|Default|Getmain_bodymesh))
  (Utilities|FlowControl|Sequence
    (:then_0
      (bind _is_activated (CallFunction|Fuc#IsActivated#))
      ;[1 1 1] set material according to status
      (if _is_activated
        (Rendering|Material|SetMaterial _main_bodymesh 0 "/Game/BluePrints/CoreGameplay/Materials/M_Excited_Receiver.M_Excited_Receiver")
        (for _array_element (Collision|GetOverlappingActors "/Game/BluePrints/CoreGameplay/Note_flick.Note_flick_C" :!class /Script/Engine.Actor)
          (bind _asnote_flick (Utilities|Casting|CastToNote_flick _array_element))
          (Actor|DestroyActor _asnote_flick)
          (Default|CallGetPoint _asnote_flick))
        (else
          (Rendering|Material|SetMaterial _main_bodymesh 0 "/Engine/BasicShapes/BasicShapeMaterial.BasicShapeMaterial"))))))

(event EventBeginPlay
  (bind _output_get (Variables|Default|SetSlot (Utilities|String|Append "receiver" (Utilities|String|ToString(Integer) (Variables|Default|GetID)))))
  (CallFunction|InitStruct)
  (bind _returnvalue (SaveGame|DoesSaveGameExist _output_get))
  (if (not _returnvalue)
    (bind _returnvalue_2 (SaveGame|CreateSaveGameObject "/Game/BluePrints/CoreGameplay/Receiver/SG_ReceiverInit.SG_ReceiverInit_C"))
    (Variables|Default|SetSaveGameObj _returnvalue_2)
    (Variables|/Game/BluePrints/CoreGameplay/Receiver/SG_ReceiverInit.SG_ReceiverInit_C|SetReceiverStruct%28SavegameVar%29 (Variables|Default|GetSaveGameObj) (Variables|Default|GetReceiver%20Struct))
    (SaveGame|SaveGametoSlot (Variables|Default|GetSaveGameObj) (Variables|Default|GetSlot))))

(fn ConstructionScript)

(fn Fuc#IsActivated#
  (bind _outactors (Actor|GetAllActorsOfClass "/Game/BluePrints/CoreGameplay/Head_of_player.Head_of_player_C"))
  (bind _ashead_of_player (Utilities|Casting|CastToHead_of_player (Utilities|Array|Get(acopy) _outactors)))
  (bind _output_get (Variables|Default|SetStatus (Math|Boolean|ORBoolean (and (>= (Variables|Default|GetTurnAngleMax) (.Turn (Utilities|Struct|BreakMediaPipeFaceRotation (Variables|/Game/BluePrints/CoreGameplay/Head_of_player.Head_of_player_C|GetHead%20Rotation _ashead_of_player)))) (>= (.Turn (Utilities|Struct|BreakMediaPipeFaceRotation (Variables|/Game/BluePrints/CoreGameplay/Head_of_player.Head_of_player_C|GetHead%20Rotation _ashead_of_player))) (Variables|Default|GetTurnAngleMin))) (and (>= (Variables|Default|GetTiltAngleMax) (.Tilt (Utilities|Struct|BreakMediaPipeFaceRotation (Variables|/Game/BluePrints/CoreGameplay/Head_of_player.Head_of_player_C|GetHead%20Rotation _ashead_of_player)))) (>= (.Tilt (Utilities|Struct|BreakMediaPipeFaceRotation (Variables|/Game/BluePrints/CoreGameplay/Head_of_player.Head_of_player_C|GetHead%20Rotation _ashead_of_player))) (Variables|Default|GetTiltAngleMin))) (and (>= (Variables|Default|GetNodAngleMax) (.Nod (Utilities|Struct|BreakMediaPipeFaceRotation (Variables|/Game/BluePrints/CoreGameplay/Head_of_player.Head_of_player_C|GetHead%20Rotation _ashead_of_player)))) (>= (.Nod (Utilities|Struct|BreakMediaPipeFaceRotation (Variables|/Game/BluePrints/CoreGameplay/Head_of_player.Head_of_player_C|GetHead%20Rotation _ashead_of_player))) (Variables|Default|GetNodAngleMin))))))
  (return _output_get))

(fn InitStruct
  (Variables|Default|SetReceiver%20Struct (Utilities|Struct|MakeS_receiverInfo (Transformation|GetActorTransform) (Variables|Default|GetID) (Utilities|MMakeInclusiveRange (Variables|Default|GetTiltAngleMin) (Variables|Default|GetTiltAngleMax)) (Utilities|MMakeInclusiveRange (Variables|Default|GetTurnAngleMin) (Variables|Default|GetTurnAngleMax)))))