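; MP_Pipeline is a Blueprint wrapper around a MediaPipe capture pipeline and its landmark observers.
; StartPipeline copies input, camera, resolution and overlay settings into the Pipeline and starts it when EnableAutoStart is set, with helpers to stop it and set graph nodes.
; Debug helpers draw camera and world origins, while DrawLandmarks now only returns an observer's face status, its drawing and printing left disconnected.
; BeginPlay and Tick are empty.
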(event EventBeginPlay)

(event EventTick
  (params (DeltaSeconds :type Float%20%28single-precision%29)))

(event EventEndPlay
  (params (EndPlayReason :type EEndPlayReason%20Enum :default "Destroyed")))

(fn ConstructionScript)

(fn StartPipeline
  (bind _pipeline (Variables|Default|GetPipeline))
  (if (Variables|MediaPipe|Pipeline|GetEnableAutoStart)
    (Variables|/Script/MediaPipe.MediaPipePipelineComponent|SetInputFile _pipeline (Variables|MediaPipe|Pipeline|GetInputFile))
    (Variables|/Script/MediaPipe.MediaPipePipelineComponent|SetCameraId _pipeline (Variables|MediaPipe|Pipeline|GetCamId))
    (Variables|/Script/MediaPipe.MediaPipePipelineComponent|SetCaptureApi _pipeline (Variables|MediaPipe|Pipeline|GetCaptureApi))
    (Variables|/Script/MediaPipe.MediaPipePipelineComponent|SetResX _pipeline (Variables|MediaPipe|Pipeline|GetResX))
    (Variables|/Script/MediaPipe.MediaPipePipelineComponent|SetResY _pipeline (Variables|MediaPipe|Pipeline|GetResY))
    (Variables|/Script/MediaPipe.MediaPipePipelineComponent|SetbEnableOverlay _pipeline (Variables|MediaPipe|Pipeline|GetEnableOverlay))
    (CameraShake|Start _pipeline)))

(fn StopPipeline
  (Audio|Components|Audio|Stop (Variables|Default|GetPipeline)))

(fn SetGraphNode
  (params (Node :type String))
  (Variables|/Script/MediaPipe.MediaPipePipelineComponent|SetGraphNodes (Variables|Default|GetPipeline) (Utilities|Array|MakeArray Node)))

(fn SetGraphNodes
  (params (Nodes :type Array%20of%20Strings))
  (Variables|/Script/MediaPipe.MediaPipePipelineComponent|SetGraphNodes (Variables|Default|GetPipeline) Nodes))

(fn DrawCameraOrigin
  (bind _cameraorigin (Variables|MediaPipe|Pipeline|GetCameraOrigin))
  (Class|KismetSystemLibrary|DrawDebugCoordinateSystem _cameraorigin "-90.000000,0.000000,0.000000" 1e+01 0.0 0.0)
  (Rendering|Debug|DrawDebugBox :Center (+ _cameraorigin "0,50.000000,-50.000000") :Extent "5.000000,50.000000,50.000000"))

(fn DrawWorldOrigin
  (bind _worldorigin (Variables|MediaPipe|Pipeline|GetWorldOrigin))
  (Class|KismetSystemLibrary|DrawDebugCoordinateSystem _worldorigin "0, 0, 0" 1e+01 0.0 0.0)
  (Rendering|Debug|DrawDebugBox _worldorigin "100.000000,100.000000,100.000000" "(R=0.000000,G=0.000000,B=0.000000,A=1.000000)" "0, 0, 0" 0.0 0.0))

(fn DrawLandmarks
  (params (Observer :type Media%20Pipe%20Landmark%20Observer%20Component%20Object%20Reference) (ObjectId :type Integer) (Origin :type Vector) (PrimitiveScale :type Float%20%28single-precision%29) (PrimitiveColor :type Linear%20Color%20Structure))
  (Utilities|IsValid Observer
    (:Is%20Valid
      (if (Class|MediaPipeObserverComponent|HaveDetections Observer)
        (return (Class|MediaPipeLandmarkObserverComponent|GetFaceStatus Observer ObjectId))))))