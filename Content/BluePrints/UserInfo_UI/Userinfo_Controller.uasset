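; User-stats tracker actor that records playtime, played songs and head tilt into the game instance during a song.
; BeginPlay caches the Head_of_player actor and adds the current song to today's played list.
; Tick grows total playtime, adds time to a tilt-angle histogram, and rebuilds today's info from the date-keyed PunchInTimes entry plus frame time.
; It saves nothing itself, and the loaded UserInfo save goes unused.
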(event EventBeginPlay
  (bind _returnvalue (Actor|GetActorOfClass "/Game/BluePrints/CoreGameplay/Head_of_player.Head_of_player_C"))
  (Variables|Default|SetHeadOfPlayer _returnvalue)
  (SaveGame|LoadGamefromSlot "UserInfo")
  (bind _gi (CallFunction|GFuncGetGI))
  (bind _output_get (Variables|Default|SetPlayed%20Songs (.PlayedSongs (Utilities|Struct|BreakS_UserInfo (Variables|/Game/BluePrints/MUNECK_GI.MUNECK_GI_C|GetTodayUserInfo _gi)))))
  (Utilities|Array|AddUnique _output_get (Variables|/Game/BluePrints/MUNECK_GI.MUNECK_GI_C|GetSongName _gi))
  (Variables|/Game/BluePrints/MUNECK_GI.MUNECK_GI_C|SetTodayUserInfo _gi (Utilities|Struct|MakeS_UserInfo (.PlayTime (Utilities|Struct|BreakS_UserInfo (Variables|/Game/BluePrints/MUNECK_GI.MUNECK_GI_C|GetTodayUserInfo _gi))) (Variables|Default|GetPlayed%20Songs))))

(event Collision|EventActorBeginOverlap
  (params (OtherActor :type Actor%20Object%20Reference)))

(event EventTick
  (params (DeltaSeconds :type Float%20%28single-precision%29))
  (CallFunction|UpdatePlaytime DeltaSeconds)
  (CallFunction|UpdateAngles DeltaSeconds)
  (bind _gi (CallFunction|GFuncGetGI))
  (Variables|/Game/BluePrints/MUNECK_GI.MUNECK_GI_C|SetTodayUserInfo _gi (Utilities|Struct|MakeS_UserInfo (+ (.PlayTime (Utilities|Struct|BreakS_UserInfo (.Value (Utilities|Map|Find (Variables|/Game/BluePrints/MUNECK_GI.MUNECK_GI_C|GetPunchInTimes _gi) (Class|KismetMathLibrary|Today))))) DeltaSeconds) (.PlayedSongs (Utilities|Struct|BreakS_UserInfo (.Value (Utilities|Map|Find (Variables|/Game/BluePrints/MUNECK_GI.MUNECK_GI_C|GetPunchInTimes _gi) (Class|KismetMathLibrary|Today))))))))

(event EventEndPlay
  (params (EndPlayReason :type EEndPlayReason%20Enum :default "Destroyed"))
  (CallFunction|GFuncGetGI))

(fn ConstructionScript)

(fn UpdatePlaytime
  (params (DeltaSeconds :type Float%20%28single-precision%29))
  (bind _gi (CallFunction|GFuncGetGI))
  (Variables|/Game/BluePrints/MUNECK_GI.MUNECK_GI_C|SetTotalPlaytime _gi (+ (Variables|/Game/BluePrints/MUNECK_GI.MUNECK_GI_C|GetTotalPlaytime _gi) DeltaSeconds)))

(fn UpdateAngles
  (params (DeltaSeconds :type Float%20%28single-precision%29))
  (bind _headofplayer (Variables|Default|GetHeadOfPlayer))
  (bind _head_rotation (Variables|/Game/BluePrints/CoreGameplay/Head_of_player.Head_of_player_C|GetHead%20Rotation _headofplayer))
  (bind _tilt (Utilities|Struct|BreakMediaPipeFaceRotation _head_rotation))
  (bind _returnvalue (Math|Float|MapRangeClamped _tilt 0.0 3.0 1.8e+02 0.0))
  (bind _returnvalue_2 (Math|Float|Round _returnvalue))
  (bind _gi (CallFunction|GFuncGetGI))
  (Utilities|Array|SetArrayElem (Variables|/Game/BluePrints/MUNECK_GI.MUNECK_GI_C|GetTiltedAngles _gi) _returnvalue_2 (+ (Utilities|Array|Get(acopy) (Variables|/Game/BluePrints/MUNECK_GI.MUNECK_GI_C|GetTiltedAngles _gi) _returnvalue_2) DeltaSeconds)))