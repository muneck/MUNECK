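; Legacy pawn-style node Blueprint that travels along a set direction and scales its body by how far it has moved toward a target.
; Each Tick forces movement input along SpeedOfNode, then recomputes Progress as distance from StartPos over the StartPos-to-TargetPos distance, capped at one.
; Progress then multiplies ScaleVector to set MainBody's relative scale, so size follows travel completion.
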(event EventBeginPlay)

(event Collision|EventActorBeginOverlap
  (params (OtherActor :type Actor%20Object%20Reference)))

(event EventTick
  (params (DeltaSeconds :type Float%20%28single-precision%29))
  (Pawn|Input|AddMovementInput (Variables|Default|Getspeed_of_Node) 1.0 true)
  (CallFunction|Func#updateProgress#)
  (CallFunction|UpadateScale))

(fn ConstructionScript)

(fn Func#updateProgress#
  (Variables|Default|Setprogress (Math|Float|Min(Float) (/ (Math|Vector|VectorLength (- (Transformation|GetActorLocation) (Variables|Default|GetStart%20Pos))) (Math|Vector|VectorLength (- (Variables|Default|GetTarget%20Pos) (Variables|Default|GetStart%20Pos)))) 1.0)))

(fn UpadateScale
  (Transformation|SetRelativeScale3D (Variables|Default|GetMain%20body) (* (LocalVariables|Getscale%20vector) (Variables|Default|Getprogress))))