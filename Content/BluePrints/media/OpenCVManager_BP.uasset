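; OpenCV manager Blueprint that feeds a camera material into a render target, extending its parent's BeginPlay and Tick.
; Each Tick draws CameraMatRaw into CameraRenderTarget when both are valid.
; An unconnected setup chain would create raw and post screen materials, open the CameraID capture device in a media player, and bind CameraTexture2D to the post material after a short delay.
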(event EventBeginPlay
  (|CallParentFunction))

(event EventTick
  (params (DeltaSeconds :type Float%20%28single-precision%29))
  (bind _camera_rendertarget (Variables|Default|GetCamera_RenderTarget))
  (bind _camera_matraw (Variables|Default|GetCamera_MatRaw))
  (|CallParentFunction DeltaSeconds)
  (Utilities|IsValid _camera_rendertarget
    (:Is%20Valid
      (Utilities|IsValid _camera_matraw
        (:Is%20Valid
          (Rendering|DrawMaterialtoRenderTarget _camera_rendertarget _camera_matraw))))))

(fn ConstructionScript)