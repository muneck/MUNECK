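; Game instance for the MUNECK rhythm game, holding the song repository, score state and note orientation.
; On Init it loads user JSON, scans Content/Charts, and parses each song's meta.json into song and difficulty entries for the repository UI list.
; It also precomputes note yaw for five rails from their viewport start and end points mapped to world space.
; ResetScore clears score and combos, then rescans charts; user score handling is unfinished.
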(event EventInit
  (Utilities|FlowControl|Sequence
    (:then_0
      (CallFunction|ParseUserData))
    (:then_1
      (CallFunction|ReadRepoData))
    (:then_2
      (for _index (range -2 2)
        (bind _v_in_levels (CallFunction|VportScaled2map (.Value (Utilities|Map|Find (Variables|ConstsMapping|GetRail_StartPos) _index))))
        (bind _v_in_levels_2 (CallFunction|VportScaled2map (.Value (Utilities|Map|Find (Variables|ConstsMapping|GetRail_EndPos) _index))))
        (Utilities|Map|Add (Variables|ConstsMapping|GetNoteTransform) _index (Math|Transform|MakeTransform "0, 0, 0" (Math|Rotator|MakeRotator 0.0 0.0 (- 9e+01 (Class|KismetMathLibrary|DegAtan (/ (.Y (Math|Vector|BreakVector (- _v_in_levels_2 _v_in_levels))) (* -1 (.X (Math|Vector|BreakVector (- _v_in_levels_2 _v_in_levels))))))))))))))

(fn ResetScore
  (Variables|inGame|GlobalVariables|SetScore 0.0)
  (Variables|inGame|GlobalVariables|SetCombo 0)
  (Variables|inGame|GlobalVariables|SetMaxCombo 0)
  (CallFunction|ReadRepoData))

(fn ParseSongMetadata
  (params (song%20name :type String))
  (bind _songdifficultylist (Variables|inGame|Datas|GetSongDifficultyLIst))
  (LocalVariables|Setsong%20directory%20path%28L%29 (Utilities|String|Append (Class|KismetSystemLibrary|GetProjectContentDirectory) "Charts/" song%20name))
  (bind _ijsonobject (Class|IJsonBlueprintFunctionLibrary|LoadJsonStringfromFile (Utilities|String|Append (LocalVariables|Getsong%20directory%20path%28L%29) "/meta.json")))
  (bind _outstring (Class|IJsonObject|TryGetStringField _ijsonobject "Name"))
  (bind _outstring_2 (Class|IJsonObject|TryGetStringField _ijsonobject "MusicFile"))
  (bind _outstring_3 (Class|IJsonObject|TryGetStringField _ijsonobject "IllustrationFile"))
  (bind _outstring_4 (Class|IJsonObject|TryGetStringField _ijsonobject "Artist"))
  (bind _outstring_5 (Class|IJsonObject|TryGetStringField _ijsonobject "Illustrator"))
  (bind _outnumber (Class|IJsonObject|TryGetNumberField _ijsonobject "ChartOffset"))
  (bind _output_get (Variables|inGame|Datas|SetSongInfo (Utilities|Struct|MakeS_SongInfo _outstring _outstring_2 _outstring_3 _outstring_4 _outstring_5 _outnumber)))
  (bind _outarray (Class|IJsonObject|TryGetJsonObjectArrayField _ijsonobject "Difficulties"))
  (for _array_element _outarray
    (bind _outstring_6 (Class|IJsonObject|TryGetStringField _array_element "DifficultyName"))
    (bind _outnumber_2 (Class|IJsonObject|TryGetNumberField _array_element "Difficulty"))
    (bind _outstring_7 (Class|IJsonObject|TryGetStringField _array_element "Chart"))
    (bind _outstring_8 (Class|IJsonObject|TryGetStringField _array_element "ChartDesigner"))
    (Utilities|Array|Add (Variables|inGame|Datas|GetSongDifficultyLIst) (Utilities|Struct|MakeS_SongDifficultyInfo _outstring_6 (Math|Float|Truncate _outnumber_2) _outstring_7 _outstring_8)))
  ;[1 1 1] due to the default value
  (Utilities|Array|RemoveIndex _songdifficultylist)
  (return _songdifficultylist _output_get))

(fn ReadRepoData
  (bind _returnvalue (Class|KismetSystemLibrary|GetProjectContentDirectory))
  (bind _returnvalue_2 (Utilities|String|Append _returnvalue "Charts/"))
  (Development|PrintString _returnvalue_2 true true "(R=0.000000,G=0.660000,B=1.000000,A=1.000000)" 12.0)
  (Utilities|MCheckExist _returnvalue_2 true false)
  (bind _returnvalue_3 (Class|CFLFolderManager|FindFilesRecursive _returnvalue_2 "*" false true))
  (for _array_element _returnvalue_3
    (bind _output_get (LocalVariables|Setsong%20name%28iter%29 (.RightS (Utilities|String|Split _array_element "Content/Charts/" "CaseSensitive"))))
    (Development|PrintString _output_get true true "(R=0.264583,G=1.000000,B=0.382222,A=1.000000)" 12.0)
    (bind (_songdifficultylist _song_info) (CallFunction|ParseSongMetadata _output_get))
    (Utilities|Array|Add (Variables|User|GetRepoUI_SonginfoList) (Utilities|Struct|MakeS_Repository_UI_Songinfo _output_get _song_info 0 _songdifficultylist))))

(fn UpdateUserData
  ;[1 1 1] To BE Implement
)

(fn ParseUserData
  ;[1 1 1] WIP(next EA)
  (Utilities|FlowControl|Sequence
    (:then_0
      (bind _ijsonobject (Class|IJsonBlueprintFunctionLibrary|LoadJsonStringfromFile (Utilities|String|Append (Class|KismetSystemLibrary|GetProjectContentDirectory) "/User/usr.json")))
      (Variables|User|Data|SetUserData%28json%29 _ijsonobject))))