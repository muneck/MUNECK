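; Component that holds the layout data for five note rails, indexed from -2 to 2 around a center rail.
; On BeginPlay it fills three maps: normalized 2D start positions, 2D end positions, and note transforms that differ only in rotation.
; Lookup functions take a rail index and return the matching position or transform with a success flag.
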(event EventBeginPlay
  (Variables|Default|SetRail_EndPos (Utilities|Map|MakeMap -2 "(X=0.730000,Y=0.339000)" -1 "(X=0.600000,Y=0.420000)" 0 "(X=0.564000,Y=0.500000)" 1 "(X=0.600000,Y=0.580000)" 2 "(X=0.730000,Y=0.661000)"))
  (Variables|Default|SetRail_StartPos (Utilities|Map|MakeMap -2 "(X=0.450000,Y=0.000000)" -1 "(X=0.000000,Y=0.180000)" 0 "(X=0.000000,Y=0.500000)" 1 "(X=0.000000,Y=0.900000)" 2 "(X=0.450000,Y=1.000000)"))
  (Variables|Default|SetNoteTransform (Utilities|Map|MakeMap -2 (Math|Transform|MakeTransform "0, 0, 0" "0,-70.000000, 0") -1 (Math|Transform|MakeTransform "0, 0, 0" "0,-40.000000, 0") 0 (Math|Transform|MakeTransform "0, 0, 0") 1 (Math|Transform|MakeTransform "0, 0, 0" "0,40.000000, 0") 2 (Math|Transform|MakeTransform "0, 0, 0" "0,70.000000, 0"))))

(event EventTick
  (params (DeltaSeconds :type Float%20%28single-precision%29)))

(fn Func#getEndposOfRail#
  (params (Rail :type Integer))
  (bind _rail_endpos (Variables|Default|GetRail_EndPos))
  (bind (_value _returnvalue) (Utilities|Map|Find _rail_endpos Rail))
  (return _value _returnvalue))

(fn Func#getStartposOfRail#0
  (params (Rail :type Integer))
  (bind _rail_startpos (Variables|Default|GetRail_StartPos))
  (bind (_value _returnvalue) (Utilities|Map|Find _rail_startpos Rail))
  (return _value _returnvalue))

(fn Func#getTransformOfRail#0
  (params (Rail :type Integer))
  (bind _notetransform (Variables|Default|GetNoteTransform))
  (bind (_value _returnvalue) (Utilities|Map|Find _notetransform Rail))
  (return _value _returnvalue))