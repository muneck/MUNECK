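; Blueprint function library of global helpers for fetching core game objects and printing timing debug info.
; Two getters return the game instance cast to MUNECK_GI and the first BP_GameStateManager actor found in the world.
; Two print helpers, gated by an Enables flag, show the game instance's song time against BP_music_loader's actual sound wave playback time, or its controller tick, with a caller-supplied prefix.
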(fn GFuncGetGI
  (bind _asmuneck_gi (Utilities|Casting|CastToMUNECK_GI (Game|GetGameInstance (LocalVariables|Get__WorldContext))))
  (return _asmuneck_gi))

(fn GfuncGetGSM
  (bind _returnvalue (Actor|GetActorOfClass (LocalVariables|Get__WorldContext) "/Game/BluePrints/CoreGameplay/BP_GameStateManager.BP_GameStateManager_C"))
  (return _returnvalue))

(fn GfuncPrintSongTime
  (params (prefix :type Text))
  (bind ___worldcontext (LocalVariables|Get__WorldContext))
  (if (LocalVariables|Getenables)
    (bind _gi (CallFunction|GFuncGetGI ___worldcontext))
    (bind _returnvalue (Actor|GetActorOfClass ___worldcontext "/Game/BluePrints/CoreGameplay/Load_Music/BP_music_loader.BP_music_loader_C"))
    (Development|PrintString ___worldcontext (Utilities|String|ToString(Text) (Utilities|Text|FormatText "{prefix}: Song time={GITime}/{RealTIme}" prefix (Variables|/Game/BluePrints/MUNECK_GI.MUNECK_GI_C|Getsong_time _gi) (Class|ImportedSoundWave|GetPlaybackTime (Variables|/Game/BluePrints/CoreGameplay/Load_Music/BP_music_loader.BP_music_loader_C|GetImported%20Sound%20Wave _returnvalue)))) true true "(R=1.000000,G=0.384786,B=0.354167,A=1.000000)" 2e+01)))

(fn GfuncPrintControllerTickTime
  (params (prefix :type Text))
  (bind ___worldcontext (LocalVariables|Get__WorldContext))
  (if (LocalVariables|Getenables)
    (bind _gi (CallFunction|GFuncGetGI ___worldcontext))
    (Development|PrintString ___worldcontext (Utilities|String|ToString(Text) (Utilities|Text|FormatText "{prefix}: Controller tick={Time}" prefix (Variables|/Game/BluePrints/MUNECK_GI.MUNECK_GI_C|GetControllerTick _gi))) true true "(R=1.000000,G=0.960381,B=0.041773,A=1.000000)" 2e+01)))