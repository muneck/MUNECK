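; Scoring function library that converts a total score into a letter grade and a note's performance into a rating, apparently for a rhythm game.
; GetGradeFromScore maps fixed score bands to S through C, with μ for exactly 10485760 and F as fallback.
; GetNoteRating sorts performance into four tiers from perfect to zero.
; It also increments that tier's count in the game instance's FinalNote map, so each call has a side effect.
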(fn GetGradefromScore
  (params (Score :type Float%20%28single-precision%29))
  (if (== Score 1.048576e+07)
    (return "μ")
    (elif (Math|Float|InRange(Float) Score 9961472.0 1.048576e+07 true false)
      (return "S")
      (elif (Math|Float|InRange(Float) Score 9437184.0 9961472.0 true false)
        (return "A")
        (elif (Math|Float|InRange(Float) Score 8388608.0 9437184.0 true false)
          (return "B")
          (elif (Math|Float|InRange(Float) Score 7340032.0 8388608.0 true false)
            (return "C")
            (else
              (return "F"))))))))

(fn GetNoteRating
  (params (Performance :type Float%20%28single-precision%29))
  (if (== Performance 1.0)
    (bind _gi (CallFunction|GFuncGetGI))
    (Utilities|Map|Add (Variables|/Game/BluePrints/MUNECK_GI.MUNECK_GI_C|GetfinalNote _gi) "NewEnumerator0" (+ (.Value (Utilities|Map|Find (Variables|/Game/BluePrints/MUNECK_GI.MUNECK_GI_C|GetfinalNote _gi) "NewEnumerator0")) 1))
    (return "NewEnumerator0")
    (elif (Math|Float|InRange(Float) Performance 0.8 1.0 true false)
      (bind _gi_2 (CallFunction|GFuncGetGI))
      (Utilities|Map|Add (Variables|/Game/BluePrints/MUNECK_GI.MUNECK_GI_C|GetfinalNote _gi_2) "NewEnumerator1" (+ (.Value (Utilities|Map|Find (Variables|/Game/BluePrints/MUNECK_GI.MUNECK_GI_C|GetfinalNote _gi_2) "NewEnumerator1")) 1))
      (return "NewEnumerator1")
      (elif (Math|Float|InRange(Float) Performance 0.0 0.8 false false)
        (bind _gi_3 (CallFunction|GFuncGetGI))
        (Utilities|Map|Add (Variables|/Game/BluePrints/MUNECK_GI.MUNECK_GI_C|GetfinalNote _gi_3) "NewEnumerator2" (+ (.Value (Utilities|Map|Find (Variables|/Game/BluePrints/MUNECK_GI.MUNECK_GI_C|GetfinalNote _gi_3) "NewEnumerator2")) 1))
        (return "NewEnumerator2")
        (elif (== Performance 0.0)
          (bind _gi_4 (CallFunction|GFuncGetGI))
          (Utilities|Map|Add (Variables|/Game/BluePrints/MUNECK_GI.MUNECK_GI_C|GetfinalNote _gi_4) "NewEnumerator3" (+ (.Value (Utilities|Map|Find (Variables|/Game/BluePrints/MUNECK_GI.MUNECK_GI_C|GetfinalNote _gi_4) "NewEnumerator3")) 1))
          (return "NewEnumerator3"))))))