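; POS_convert is a Blueprint function set that converts positions between viewport coordinates and level map space bounded by upper-left and down-right screen corners.
; Viewport-to-map functions interpolate across those bounds with a Z term of 150, from pixel or pre-scaled input; only the pixel version swaps X and Y.
; The inverse maps level positions to pixels, and a scaling helper normalizes by the same doubled viewport size.
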(fn Vport2map
  (params (v%20in%20viewport :type Vector%202D%20Structure))
  (bind (_x _y) (Math|Vector2D|BreakVector2D v%20in%20viewport))
  (bind _scr_dr (LocalVariables|Getscr_DR))
  (bind _scr_ul (LocalVariables|Getscr_UL))
  (bind _returnvalue (- _scr_dr _scr_ul))
  (bind (_x_2 _y_2) (Math|Vector|BreakVector _returnvalue))
  (bind _output_get (LocalVariables|SetSIZE (Math|Conversions|ToVector2D(Vector) (* (Math|Conversions|ToVector(Vector2D) (Viewport|GetViewportSize (LocalVariables|Get__WorldContext))) 2.0))))
  (return (+ (Math|Vector|MakeVector (* (/ _y (.Y (Math|Vector2D|BreakVector2D _output_get))) _x_2) (* _y_2 (/ _x (.X (Math|Vector2D|BreakVector2D _output_get)))) 1.5e+02) (LocalVariables|Getscr_UL))))

(fn Map2vport
  (params (v%20in%20level :type Vector))
  (bind _scr_ul_0 (LocalVariables|Getscr_UL_0))
  (bind _scr_dr_0 (LocalVariables|Getscr_DR_0))
  (bind _scr_ul_0_2 (LocalVariables|Getscr_UL_0))
  (bind _returnvalue (- v%20in%20level _scr_ul_0))
  (bind _returnvalue_2 (- _scr_dr_0 _scr_ul_0_2))
  (bind (_x _y) (Math|Vector|BreakVector _returnvalue))
  (bind (_x_2 _y_2) (Math|Vector|BreakVector _returnvalue_2))
  (bind _output_get (LocalVariables|SetSIZE (Math|Conversions|ToVector2D(Vector) (* (Math|Conversions|ToVector(Vector2D) (Viewport|GetViewportSize (LocalVariables|Get__WorldContext))) 2.0))))
  (return (Math|Vector2D|MakeVector2D (* (.X (Math|Vector2D|BreakVector2D _output_get)) (/ _x _x_2)) (* (.Y (Math|Vector2D|BreakVector2D _output_get)) (/ _y _y_2)))))

(fn VportScaled2map
  (params (v%20in%20viewport :type Vector%202D%20Structure))
  (bind (_x _y) (Math|Vector2D|BreakVector2D v%20in%20viewport))
  (bind _scr_dr (LocalVariables|Getscr_DR))
  (bind _scr_ul (LocalVariables|Getscr_UL))
  (bind _returnvalue (- _scr_dr _scr_ul))
  (bind (_x_2 _y_2) (Math|Vector|BreakVector _returnvalue))
  (return (+ (Math|Vector|MakeVector (* _x _x_2) (* _y_2 _y) 1.5e+02) (LocalVariables|Getscr_UL))))

(fn VportScaling
  (params (Origin%20Pos :type Vector%202D%20Structure))
  (bind _output_get (LocalVariables|SetSIZE (Math|Conversions|ToVector2D(Vector) (* (Math|Conversions|ToVector(Vector2D) (Viewport|GetViewportSize (LocalVariables|Get__WorldContext))) 2.0))))
  (return (/ Origin%20Pos _output_get)))