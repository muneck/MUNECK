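; Actor controller that supplies song data to the repository (song list) UI in what appears to be a music game.
; GetDisplayNumber maps a slot location to a wrapped, 1-based song number using the widget's relative and absolute sequence.
; Lookup functions read name, artist, top score and difficulty from RepositorySonginfo, capping too-high modes at the last difficulty.
; The difficulty lookup indexes by DisplayNumber directly, whereas the info lookup subtracts one.
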(event EventBeginPlay)

(event Collision|EventActorBeginOverlap
  (params (OtherActor :type Actor%20Object%20Reference)))

(event EventTick
  (params (DeltaSeconds :type Float%20%28single-precision%29)))

(fn ConstructionScript)

(fn GetDisplayNumber
  (params (location :type Integer))
  (bind _repositorywidget (Variables|Default|GetrepositoryWidget))
  (bind _totalsongnumber (Variables|Default|GetTotalSongNumber))
  (bind _output_get (Variables|Default|SetdisplayNumber (Math|Integer|%(Integer) (+ (- location (Variables|/Game/BluePrints/Repository_UI/Repository_Widget.Repository_Widget_C|Getrelative%20sequence _repositorywidget)) (Variables|/Game/BluePrints/Repository_UI/Repository_Widget.Repository_Widget_C|Getabsolute%20sequence _repositorywidget)) (Variables|Default|GetTotalSongNumber))))
  (if (== _output_get 0)
    (Variables|Default|SetdisplayNumber _totalsongnumber)
    (elif (< (Variables|Default|GetdisplayNumber) 0)
      (Variables|Default|SetdisplayNumber (+ (Variables|Default|GetdisplayNumber) _totalsongnumber))))
  (return (Variables|Default|GetdisplayNumber)))

(fn GetInfofromDisplayNumber
  (params (Display%20number :type Integer))
  (bind _returnvalue (- Display%20number 1))
  (bind _repository_songinfo (Variables|Default|GetRepository%20Songinfo))
  (bind _output (Utilities|Array|Get(acopy) _repository_songinfo _returnvalue))
  (bind (_song_info _song_topscore) (Utilities|Struct|BreakS_Repository_UI_Songinfo _output))
  (bind (_displayname _musicfile _illustrationfile _artist) (Utilities|Struct|BreakS_SongInfo _song_info))
  (return _displayname _artist (Utilities|String|ToString(Text) _song_topscore)))

(fn GetInfoforDifficultywithDisplayNumber
  (params (Display%20Number :type Integer) (Mode%20Number :type Integer))
  (bind _repository_songinfo (Variables|Default|GetRepository%20Songinfo))
  (bind _output (Utilities|Array|Get(acopy) _repository_songinfo Display%20Number))
  (bind _song_difficulty_list (Utilities|Struct|BreakS_Repository_UI_Songinfo _output))
  (bind _returnvalue (Utilities|Array|Length _song_difficulty_list))
  (if (> Mode%20Number _returnvalue)
    (Variables|Default|SetDifficulty%20number%20index (- _returnvalue 1))
    (else
      (Variables|Default|SetDifficulty%20number%20index (- Mode%20Number 1))))
  (return _returnvalue (.DifficultyName (Utilities|Struct|BreakS_SongDifficultyInfo (Utilities|Array|Get(acopy) _song_difficulty_list (Variables|Default|GetDifficulty%20number%20index)))) (Utilities|String|ToString(Integer) (.Difficulty (Utilities|Struct|BreakS_SongDifficultyInfo (Utilities|Array|Get(acopy) _song_difficulty_list (Variables|Default|GetDifficulty%20number%20index)))))))