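; BP_catcher is an actor that follows the mouse cursor and destroys any Main_Nodes actor that begins overlapping its capsule.
; Each tick it converts the viewport mouse position through Vport2map and moves there without sweeping.
; MouseX and MouseY axis events also accumulate a scaled Position variable, which the movement does not read.
; The POSTransform function is a stub returning a zero vector.
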(event OnComponentBeginOverlap(Capsule)
  (params (OverlappedComponent :type Primitive%20Component%20Object%20Reference) (OtherActor :type Actor%20Object%20Reference) (OtherComp :type Primitive%20Component%20Object%20Reference) (OtherBodyIndex :type Integer) (bFromSweep :type Boolean) (SweepResult :type Hit%20Result%20Structure%20%28by%20ref%29))
  ;[1 1 1] collision destroy
  (Development|PrintString (Utilities|GetDisplayName OtherActor))
  (Utilities|Casting|CastToMain_Nodes OtherActor)
  (Actor|DestroyActor OtherActor))

(event EventBeginPlay)

(event Collision|EventActorBeginOverlap
  (params (OtherActor :type Actor%20Object%20Reference)))

(event EventTick
  (params (DeltaSeconds :type Float%20%28single-precision%29))
  (bind _returnvalue (Class|WidgetLayoutLibrary|GetMousePositiononViewport))
  (bind _v_in_levels (CallFunction|Vport2map _returnvalue))
  (Transformation|SetActorLocation _v_in_levels false false)
  (Development|PrintString (Utilities|String|ToString(Vector2d) _returnvalue) false false))

(event Input|MouseEvents|MouseX
  (params (AxisValue :type Float%20%28single-precision%29))
  ;[1 1 1] change position
  (Variables|Default|Setposition (Math|Vector|MakeVector (.X (Math|Vector|BreakVector (Variables|Default|Getposition))) (+ (.Y (Math|Vector|BreakVector (Variables|Default|Getposition))) (* AxisValue 1e+01)) (.Z (Math|Vector|BreakVector (Variables|Default|Getposition))))))

(event Input|MouseEvents|MouseY
  (params (AxisValue :type Float%20%28single-precision%29))
  ;[1 1 1] change position
  (Variables|Default|Setposition (Math|Vector|MakeVector (+ (.X (Math|Vector|BreakVector (Variables|Default|Getposition))) (* AxisValue 1e+01)) (.Y (Math|Vector|BreakVector (Variables|Default|Getposition))) (.Z (Math|Vector|BreakVector (Variables|Default|Getposition))))))

(fn ConstructionScript)

(fn POSTransform
  (params (vector%20in%20viewport :type Vector))
  (return "0, 0, 0"))